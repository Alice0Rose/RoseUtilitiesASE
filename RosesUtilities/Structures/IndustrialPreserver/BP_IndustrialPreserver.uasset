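; Industrial Preserver item-container structure that automatically pulls items from same-team whitelisted structures and shows a coldness effect while active.
; On BeginPlay the server loads range, whitelist, blacklist and extra allowed items from the RosesUtilities global actor, then starts a looping collection timer.
; While activated and team-toggled on via a multi-use entry, it scans its platform saddle's structures, or otherwise octree-overlaps nearby ones, transferring non-blacklisted items.
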(event EventParentFirstBeginPlay
  (Utilities|FlowControl|Sequence
    (:then_0
      ;[1 1 1] Gets range, auto-collect structures, and extra allowed items config
      (Class|KismetSystemLibrary|IsRunningonServer
        (:Yes
          (bind _globalactor (CallFunction|RUGetGlobalActor self))
          (Variables|Default|SeteffectRange (* 300 (Variables|/Game/Mods/RosesUtilities/RosesUtilities_GlobalActor.RosesUtilities_GlobalActor_C|GetIndustrialPreserverAutoCollectRange _globalactor)) true)
          (Variables|Default|SetautoCollectStructureWhitelist (Variables|/Game/Mods/RosesUtilities/RosesUtilities_GlobalActor.RosesUtilities_GlobalActor_C|GetIndustrialPreserverAutoCollectStructureWhitelist _globalactor) false)
          (Utilities|Array|AppendArray (Variables|/Script/ShooterGame.PrimalInventoryComponent|GetRemoteAddItemOnlyAllowItemClasses (Variables|Default|GetMyInventoryComponent)) (Variables|/Game/Mods/RosesUtilities/RosesUtilities_GlobalActor.RosesUtilities_GlobalActor_C|GetIndustrialPreserverAdditionalMeatItems _globalactor))
          (Variables|Default|SetautoCollectItemBlacklist (Variables|/Game/Mods/RosesUtilities/RosesUtilities_GlobalActor.RosesUtilities_GlobalActor_C|GetIndustrialPreserverAutoCollectItemBlacklist _globalactor)))))
    (:then_1
      ;[1 1 1] Restores saved visibility
      (CallFunction|OnRepEffectRange)
      (CallFunction|OnRepIsActivated))
    (:then_2
      ;[1 1 1] Starts item collect scan loop
      (Class|KismetSystemLibrary|IsRunningonServer
        (:Yes
          (Utilities|FlowControl|Delay 0.6)
          (Utilities|Time|SetTimerbyFunctionName 0 "AutoCollectItems" 6e+01 true))))))

(fn ConstructionScript
  (|CallParentFunction))

(fn BPTryMultiUse
  (params (ForPC :type Player%20Controller%20Object%20Reference) (UseIndex :type Integer))
  (|CallParentFunction ForPC UseIndex)
  (Utilities|FlowControl|Sequence
    (:then_0
      (switch string (Utilities|String|ToString(Integer) UseIndex)
        (:90314
          ;[1 1 1] Toggles auto-collect
          (Variables|Default|SetisAutoCollectActive (not (Variables|Default|GetisAutoCollectActive)) true))))
    (:then_1
      (return true))))

(fn BPGetMultiUseEntries
  (params (ForPC :type Player%20Controller%20Object%20Reference) (MultiUseEntries :type Array%20of%20Multi%20Use%20Entry%20Structures))
  (bind _isautocollectactive (Variables|Default|GetisAutoCollectActive))
  (bind _returnvalue (|CallParentFunction ForPC MultiUseEntries))
  (LocalVariables|SettempMultiUseEntries _returnvalue)
  (if (== (Variables|Default|GetTargetingTeam) (Variables|/Script/Engine.Actor|GetTargetingTeam ForPC))
    (Utilities|FlowControl|Sequence
      (:then_0
        ;[1 1 1] Adds a MultiUse entry to toggle auto collect
        (Utilities|Array|Add (LocalVariables|GettempMultiUseEntries) (Utilities|Struct|MakeMultiUseEntry 0 (Utilities|String|SelectString "Auto-Collect [Enabled]" "Auto-Collect [Disabled]" _isautocollectactive) 90314 -10000 false false false false false false false false false true false false false false 0 "(B=175,G=175,R=175,A=255)" (Math|Conversions|ToColor(LinearColor) (Math|Color|SelectColor "(R=0.250000,G=1.000000,B=0.250000,A=1.000000)" "(R=1.000000,G=0.250000,B=0.250000,A=1.000000)" _isautocollectactive)))))
      (:then_1
        (return (LocalVariables|GettempMultiUseEntries))))
    (else
      (return (LocalVariables|GettempMultiUseEntries)))))

(fn AutoCollectItems
  (bind _saddledino (Variables|Default|GetSaddleDino))
  (Class|KismetSystemLibrary|IsRunningonServer
    (:Yes
      ;[1 1 1] Disables if range is 0
      (if (> (Variables|Default|GeteffectRange) 0.0)
        ;[1 1 1] Only collects if enabled and activated
        (if (and (Variables|Default|GetisAutoCollectActive) (Variables|Default|GetisActivated))
          ;[1 1 1] Only gets structures from platform saddle if on a platform saddle
          (Utilities|IsValid _saddledino
            (:Is%20Valid
              ;[1 1 1] Transfers resources to collect from all structures on the current platform saddle
              (for _array_element (Variables|/Script/ShooterGame.PrimalDinoCharacter|GetSaddleStructures _saddledino)
                (if (and (== (Variables|/Script/Engine.Actor|GetTargetingTeam (.MyStructure (Utilities|Struct|BreakPrimalSaddleStructure _array_element))) (Variables|Default|GetTargetingTeam)) (not (== (.MyStructure (Utilities|Struct|BreakPrimalSaddleStructure _array_element)) self)))
                  (bind _asprimalstructure (Utilities|Casting|CastToPrimalStructureClass (Utilities|GetClass (.MyStructure (Utilities|Struct|BreakPrimalSaddleStructure _array_element)))))
                  (if (Utilities|Array|ContainsItem (Variables|Default|GetautoCollectStructureWhitelist) _asprimalstructure)
                    (bind _asprimalstructureitemcontainer (Utilities|Casting|CastToPrimalStructureItemContainer (.MyStructure (Utilities|Struct|BreakPrimalSaddleStructure _array_element))))
                    (CallFunction|RUTransferAllItems (Variables|/Script/ShooterGame.PrimalStructureItemContainer|GetMyInventoryComponent _asprimalstructureitemcontainer) (Variables|Default|GetMyInventoryComponent) (Variables|Default|GetautoCollectItemBlacklist) true false true false false)))))
            (:Is%20Not%20Valid
              ;[1 1 1] Gets all structures on the whitelist in range
              (for _array_element_2 (Variables|Default|GetautoCollectStructureWhitelist)
                (bind _returnvalue (Class|VictoryCore|ServerOctreeOverlapActorsClass (Class|Actor|GetWorld) (Transformation|GetActorLocation) (Variables|Default|GeteffectRange) "STRUCTURES" _array_element_2 false))
                (for _array_element_3 _returnvalue
                  ;[1 1 1] Transfers meats from all owned whitelisted structures
                  (if (== (Variables|/Script/Engine.Actor|GetTargetingTeam _array_element_3) (Variables|Default|GetTargetingTeam))
                    (bind _asprimalstructureitemcontainer_2 (Utilities|Casting|CastToPrimalStructureItemContainer _array_element_3))
                    (CallFunction|RUTransferAllItems (Variables|/Script/ShooterGame.PrimalStructureItemContainer|GetMyInventoryComponent _asprimalstructureitemcontainer_2) (Variables|Default|GetMyInventoryComponent) (Variables|Default|GetautoCollectItemBlacklist) true false true false false)))))))))))

(fn BPContainerDeactivated
  (Variables|Default|SetisActivated false true))

(fn OnRepIsActivated
  ;[1 1 1] Toggles SFX based on if structure is active
  (Rendering|SetVisibility (Variables|Default|GetColdness) (Variables|Default|GetisActivated) true))

(fn BPContainerActivated
  (Variables|Default|SetisActivated true true))