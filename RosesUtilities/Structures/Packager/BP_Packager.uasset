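; Packager structure that auto-collects resources, distributes metal and wood to forges, and packs resources into pallets via auto-craft blueprints.
; Server timers drive collection and distribution across team-owned whitelisted structures (platform saddle or octree range query) and nearby dinos, using configured range.
; Forge inventories receive even splits; enabling wood distribution disables wood pallet auto-crafting.
; Multi-use entries toggle each feature, unpack pallets, and lengthen the pickup timer once the structure has been activated.
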(event EventParentFirstBeginPlay
  (Utilities|FlowControl|Sequence
    (:then_0
      ;[1 1 1] Gets auto-collect range configs
      (Class|KismetSystemLibrary|IsRunningonServer
        (:Yes
          (bind _globalactor (CallFunction|RUGetGlobalActor self))
          (Variables|Default|SeteffectRange (* 300 (Variables|/Game/Mods/RosesUtilities/RosesUtilities_GlobalActor.RosesUtilities_GlobalActor_C|GetPackagerAutoCollectRange _globalactor)) true)
          (Variables|Default|SetautoCollectStructureWhitelist (Variables|/Game/Mods/RosesUtilities/RosesUtilities_GlobalActor.RosesUtilities_GlobalActor_C|GetPackagerAutoCollectStructureWhitelist _globalactor) true)
          (Variables|Default|SetdistributeForgeStructureWhitelist (Variables|/Game/Mods/RosesUtilities/RosesUtilities_GlobalActor.RosesUtilities_GlobalActor_C|GetPackagerDistributeStructureWhitelist _globalactor) true)
          (Variables|Default|SetdistributeForgeDinoWhitelist (Variables|/Game/Mods/RosesUtilities/RosesUtilities_GlobalActor.RosesUtilities_GlobalActor_C|GetPackagerDistributeDinoWhitelist _globalactor) true))))
    (:then_1
      ;[1 1 1] Restores saved visibility
      (CallFunction|OnRepEffectRange)
      (CallFunction|OnRepIsActivated))
    (:then_2
      ;[1 1 1] Restores wood pallet auto crafting status
      (CallFunction|OnRepIsDistributeWoodActive))
    (:then_3
      ;[1 1 1] Enables autocrafting for pallets
      (Variables|/Script/ShooterGame.PrimalInventoryComponent|SetbCheckForAutoCraftBlueprints (Variables|Default|GetMyInventoryComponent) true))
    (:then_4
      ;[1 1 1] Starts item collect and distribution loops along with unpackaging loop
      (Class|KismetSystemLibrary|IsRunningonServer
        (:Yes
          (Utilities|FlowControl|Delay 0.1)
          (Utilities|Time|SetTimerbyFunctionName 0 "AutoCollectItems" 1e+01 true)
          (Utilities|FlowControl|Delay 1.0)
          (Utilities|Time|SetTimerbyFunctionName 0 "DistributeItems" 1e+01 true))))))

(fn ConstructionScript)

(fn BPContainerActivated
  (Variables|Default|SetisActivated true true)
  (if (not (Variables|Default|GethasBeenActivated))
    (Variables|Default|SethasBeenActivated true true)))

(fn BPTryMultiUse
  (params (ForPC :type Player%20Controller%20Object%20Reference) (UseIndex :type Integer))
  (|CallParentFunction ForPC UseIndex)
  (Utilities|FlowControl|Sequence
    (:then_0
      (switch string (Utilities|String|ToString(Integer) UseIndex)
        (:90414
          ;[1 1 1] Toggles auto-collect
          (Variables|Default|SetisAutoCollectActive (not (Variables|Default|GetisAutoCollectActive)) true))
        (:90313
          ;[1 1 1] Toggles distributing metal
          (Variables|Default|SetisDistributeMetalActive (not (Variables|Default|GetisDistributeMetalActive)) true))
        (:90212
          ;[1 1 1] Toggles distributing wood
          (Variables|Default|SetisDistributeWoodActive (not (Variables|Default|GetisDistributeWoodActive)) true))
        (:90909
          ;[1 1 1] Deactivates Packager if activated and unpackages pallets
          (if (Variables|Default|GetisActivated)
            (Class|Actor|TryMultiUse ForPC 600))
          (CallFunction|UnpackagePallets))))
    (:then_1
      (return true))))

(fn BPGetMultiUseEntries
  (params (ForPC :type Player%20Controller%20Object%20Reference) (MultiUseEntries :type Array%20of%20Multi%20Use%20Entry%20Structures))
  (bind _isautocollectactive (Variables|Default|GetisAutoCollectActive))
  (bind _isdistributemetalactive (Variables|Default|GetisDistributeMetalActive))
  (bind _isdistributewoodactive (Variables|Default|GetisDistributeWoodActive))
  (bind _returnvalue (|CallParentFunction ForPC MultiUseEntries))
  (LocalVariables|SettempMultiUseEntries _returnvalue)
  (if (== (Variables|Default|GetTargetingTeam) (Variables|/Script/Engine.Actor|GetTargetingTeam ForPC))
    (Utilities|FlowControl|Sequence
      (:then_0
        (if (Variables|Default|GethasBeenActivated)
          ;[1 1 1] Extends Pickup multiuse activation timer
          (bind (_array_element _array_index) (Utilities|Array|ForEachLoopwithBreak (LocalVariables|GettempMultiUseEntries) :!label _label)
            (:LoopBody
              (if (== (.UseIndex (Utilities|Struct|BreakMultiUseEntry _array_element)) 203)
                (Utilities|Array|SetArrayElem (LocalVariables|GettempMultiUseEntries) _array_index (Utilities|Struct|MakeMultiUseEntry (.ForComponent (Utilities|Struct|BreakMultiUseEntry (Utilities|Array|Get(acopy) (LocalVariables|GettempMultiUseEntries) _array_index))) (.UseString (Utilities|Struct|BreakMultiUseEntry (Utilities|Array|Get(acopy) (LocalVariables|GettempMultiUseEntries) _array_index))) (.UseIndex (Utilities|Struct|BreakMultiUseEntry (Utilities|Array|Get(acopy) (LocalVariables|GettempMultiUseEntries) _array_index))) (.Priority (Utilities|Struct|BreakMultiUseEntry (Utilities|Array|Get(acopy) (LocalVariables|GettempMultiUseEntries) _array_index))) (.bHideFromUI (Utilities|Struct|BreakMultiUseEntry (Utilities|Array|Get(acopy) (LocalVariables|GettempMultiUseEntries) _array_index))) (.bDisableUse (Utilities|Struct|BreakMultiUseEntry (Utilities|Array|Get(acopy) (LocalVariables|GettempMultiUseEntries) _array_index))) (.bHideActivationKey (Utilities|Struct|BreakMultiUseEntry (Utilities|Array|Get(acopy) (LocalVariables|GettempMultiUseEntries) _array_index))) (.bRepeatMultiUse (Utilities|Struct|BreakMultiUseEntry (Utilities|Array|Get(acopy) (LocalVariables|GettempMultiUseEntries) _array_index))) (.bDisplayOnInventoryUI (Utilities|Struct|BreakMultiUseEntry (Utilities|Array|Get(acopy) (LocalVariables|GettempMultiUseEntries) _array_index))) (.bDisplayOnInventoryUISecondary (Utilities|Struct|BreakMultiUseEntry (Utilities|Array|Get(acopy) (LocalVariables|GettempMultiUseEntries) _array_index))) (.bHarvestable (Utilities|Struct|BreakMultiUseEntry (Utilities|Array|Get(acopy) (LocalVariables|GettempMultiUseEntries) _array_index))) (.bIsSecondaryUse (Utilities|Struct|BreakMultiUseEntry (Utilities|Array|Get(acopy) (LocalVariables|GettempMultiUseEntries) _array_index))) (.bPersistWheelOnActivation (Utilities|Struct|BreakMultiUseEntry (Utilities|Array|Get(acopy) (LocalVariables|GettempMultiUseEntries) _array_index))) (.bOverrideUseTextColor (Utilities|Struct|BreakMultiUseEntry (Utilities|Array|Get(acopy) (LocalVariables|GettempMultiUseEntries) _array_index))) (.bDisplayOnInventoryUITertiary (Utilities|Struct|BreakMultiUseEntry (Utilities|Array|Get(acopy) (LocalVariables|GettempMultiUseEntries) _array_index))) (.bClientSideOnly (Utilities|Struct|BreakMultiUseEntry (Utilities|Array|Get(acopy) (LocalVariables|GettempMultiUseEntries) _array_index))) (.bPersistWheelRequiresDirectActivation (Utilities|Struct|BreakMultiUseEntry (Utilities|Array|Get(acopy) (LocalVariables|GettempMultiUseEntries) _array_index))) (.bDrawTooltip (Utilities|Struct|BreakMultiUseEntry (Utilities|Array|Get(acopy) (LocalVariables|GettempMultiUseEntries) _array_index))) (.WheelCategory (Utilities|Struct|BreakMultiUseEntry (Utilities|Array|Get(acopy) (LocalVariables|GettempMultiUseEntries) _array_index))) (.DisableUseColor (Utilities|Struct|BreakMultiUseEntry (Utilities|Array|Get(acopy) (LocalVariables|GettempMultiUseEntries) _array_index))) (.UseTextColor (Utilities|Struct|BreakMultiUseEntry (Utilities|Array|Get(acopy) (LocalVariables|GettempMultiUseEntries) _array_index))) 3e+01 3e+01 (.ActivationSound (Utilities|Struct|BreakMultiUseEntry (Utilities|Array|Get(acopy) (LocalVariables|GettempMultiUseEntries) _array_index))) (.UseInventoryButtonStyleOverrideIndex (Utilities|Struct|BreakMultiUseEntry (Utilities|Array|Get(acopy) (LocalVariables|GettempMultiUseEntries) _array_index))) (.AdditionalButtonsIndex (Utilities|Struct|BreakMultiUseEntry (Utilities|Array|Get(acopy) (LocalVariables|GettempMultiUseEntries) _array_index)))))
                (goto _label Break))))))
      (:then_1
        ;[1 1 1] Adds a MultiUse entry to toggle auto-collect on or off
        (Utilities|Array|Add (LocalVariables|GettempMultiUseEntries) (Utilities|Struct|MakeMultiUseEntry 0 (Utilities|String|SelectString "Auto-Collect [Enabled]" "Auto-Collect [Disabled]" _isautocollectactive) 90414 -10001 false false false false false false false false false true false false false false 0 "(B=175,G=175,R=175,A=255)" (Math|Conversions|ToColor(LinearColor) (Math|Color|SelectColor "(R=0.250000,G=1.000000,B=0.250000,A=1.000000)" "(R=1.000000,G=0.250000,B=0.250000,A=1.000000)" _isautocollectactive)))))
      (:then_2
        ;[1 1 1] Adds a MultiUse entry to toggle meatl distribution on or off
        (Utilities|Array|Add (LocalVariables|GettempMultiUseEntries) (Utilities|Struct|MakeMultiUseEntry 0 (Utilities|String|SelectString "Distribute Metal [Enabled]" "Distribute Metal [Disabled]" _isdistributemetalactive) 90313 -10000 false false false false false false false false false true false false false false 0 "(B=175,G=175,R=175,A=255)" (Math|Conversions|ToColor(LinearColor) (Math|Color|SelectColor "(R=0.250000,G=1.000000,B=0.250000,A=1.000000)" "(R=1.000000,G=0.250000,B=0.250000,A=1.000000)" _isdistributemetalactive)))))
      (:then_3
        ;[1 1 1] Adds a MultiUse entry to toggle metal distribution on or off
        (Utilities|Array|Add (LocalVariables|GettempMultiUseEntries) (Utilities|Struct|MakeMultiUseEntry 0 (Utilities|String|SelectString "Distribute Wood [Enabled]" "Distribute Wood [Disabled]" _isdistributewoodactive) 90212 -9999 false false false false false false false false false true false false false false 0 "(B=175,G=175,R=175,A=255)" (Math|Conversions|ToColor(LinearColor) (Math|Color|SelectColor "(R=0.250000,G=1.000000,B=0.250000,A=1.000000)" "(R=1.000000,G=0.250000,B=0.250000,A=1.000000)" _isdistributewoodactive)))))
      (:then_4
        ;[1 1 1] Adds a MultiUse entry to unpack pallets
        (Utilities|Array|Add (LocalVariables|GettempMultiUseEntries) (Utilities|Struct|MakeMultiUseEntry 0 "Unpack Pallets" 90909 -109090 true false false false false true false false false true)))
      (:then_5
        (return (LocalVariables|GettempMultiUseEntries))))
    (else
      (return (LocalVariables|GettempMultiUseEntries)))))

(fn AutoCollectItems
  (bind _saddledino (Variables|Default|GetSaddleDino))
  (Class|KismetSystemLibrary|IsRunningonServer
    (:Yes
      ;[1 1 1] Disables if range is 0
      (if (> (Variables|Default|GeteffectRange) 0.0)
        (if (and (Variables|Default|GetisAutoCollectActive) (Variables|Default|GetisActivated))
          (Utilities|FlowControl|Sequence
            (:then_0
              ;[1 1 1] Only gets structures from platform saddle if on a platform saddle
              (Utilities|IsValid _saddledino
                (:Is%20Valid
                  ;[1 1 1] Transfers resources to collect from all structures on the current platform saddle
                  (for _array_element (Variables|/Script/ShooterGame.PrimalDinoCharacter|GetSaddleStructures _saddledino)
                    (if (and (== (Variables|/Script/Engine.Actor|GetTargetingTeam (.MyStructure (Utilities|Struct|BreakPrimalSaddleStructure _array_element))) (Variables|Default|GetTargetingTeam)) (not (== (.MyStructure (Utilities|Struct|BreakPrimalSaddleStructure _array_element)) self)))
                      (bind _asprimalstructure (Utilities|Casting|CastToPrimalStructureClass (Utilities|GetClass (.MyStructure (Utilities|Struct|BreakPrimalSaddleStructure _array_element)))))
                      (if (Utilities|Array|ContainsItem (Variables|Default|GetautoCollectStructureWhitelist) _asprimalstructure)
                        (bind _asprimalstructureitemcontainer (Utilities|Casting|CastToPrimalStructureItemContainer (.MyStructure (Utilities|Struct|BreakPrimalSaddleStructure _array_element))))
                        (CallFunction|RUTransferAllItems (Variables|/Script/ShooterGame.PrimalStructureItemContainer|GetMyInventoryComponent _asprimalstructureitemcontainer) (Variables|Default|GetMyInventoryComponent) (Variables|Default|GetautoCollectItemsToCollect_Structures) false false true false false)))))
                (:Is%20Not%20Valid
                  ;[1 1 1] Gets all valid structures to transfer from in range
                  (for _array_element_2 (Variables|Default|GetautoCollectStructureWhitelist)
                    (bind _returnvalue (Class|VictoryCore|ServerOctreeOverlapActorsClass (Class|Actor|GetWorld) (Transformation|GetActorLocation) (Variables|Default|GeteffectRange) "STRUCTURES" _array_element_2 false))
                    (for _array_element_3 _returnvalue
                      ;[1 1 1] Transfers resources to collect from all owned matching structures
                      (if (== (Variables|/Script/Engine.Actor|GetTargetingTeam _array_element_3) (Variables|Default|GetTargetingTeam))
                        (bind _asprimalstructureitemcontainer_2 (Utilities|Casting|CastToPrimalStructureItemContainer _array_element_3))
                        (CallFunction|RUTransferAllItems (Variables|/Script/ShooterGame.PrimalStructureItemContainer|GetMyInventoryComponent _asprimalstructureitemcontainer_2) (Variables|Default|GetMyInventoryComponent) (Variables|Default|GetautoCollectItemsToCollect_Structures) false false true false false)))))))
            (:then_1
              ;[1 1 1] Gets all dinos in range
              (bind _returnvalue_2 (Class|VictoryCore|ServerOctreeOverlapActorsClass (Class|Actor|GetWorld) (Transformation|GetActorLocation) (Variables|Default|GeteffectRange) "DINOPAWNS_TAMED" "/Script/ShooterGame.PrimalDinoCharacter" false))
              (for _array_element_4 _returnvalue_2
                ;[1 1 1] Transfers resources to collect from all owned dinos
                (if (== (Variables|/Script/Engine.Actor|GetTargetingTeam _array_element_4) (Variables|Default|GetTargetingTeam))
                  (bind _asprimaldinocharacter (Utilities|Casting|CastToPrimalDinoCharacter _array_element_4))
                  (CallFunction|RUTransferAllItems (Variables|/Script/ShooterGame.PrimalCharacter|GetMyInventoryComponent _asprimaldinocharacter) (Variables|Default|GetMyInventoryComponent) (Variables|Default|GetautoCollectItemsToCollect) false false true false false)
                  ;[1 1 1] Collects metal if distibuting metal is active
                  (if (Variables|Default|GetisDistributeMetalActive)
                    (CallFunction|RUTransferAllItems (Variables|/Script/ShooterGame.PrimalCharacter|GetMyInventoryComponent _asprimaldinocharacter) (Variables|Default|GetMyInventoryComponent) (Utilities|Array|MakeArray "/Game/PrimalEarth/CoreBlueprints/Resources/PrimalItemResource_Metal.PrimalItemResource_Metal_C") false false true false false)))))))))))

(fn OnRepIsActivated
  ;[1 1 1] Toggles SFX based on if structure is active
  (Rendering|SetVisibility (Variables|Default|GetParticles) (Variables|Default|GetisActivated) true))

(fn BPContainerDeactivated
  (Variables|Default|SetisActivated false true))

(fn DistributeItems
  (bind _saddledino (Variables|Default|GetSaddleDino))
  (bind _nearbyforgeinventories (LocalVariables|GetnearbyForgeInventories))
  (bind _returnvalue (Utilities|Array|Length _nearbyforgeinventories))
  (Class|KismetSystemLibrary|IsRunningonServer
    (:Yes
      ;[1 1 1] Disables if range is 0
      (if (> (Variables|Default|GeteffectRange) 0.0)
        (if (and (or (Variables|Default|GetisDistributeMetalActive) (Variables|Default|GetisDistributeWoodActive)) (Variables|Default|GetisActivated))
          (Utilities|FlowControl|Sequence
            (:then_0
              ;[1 1 1] Only gets structures from platform saddle if on a platform saddle
              (Utilities|IsValid _saddledino
                (:Is%20Valid
                  ;[1 1 1] Gets a list of all valid forge structure inventories on the current platform saddle
                  (for _array_element (Variables|/Script/ShooterGame.PrimalDinoCharacter|GetSaddleStructures _saddledino)
                    (if (and (== (Variables|/Script/Engine.Actor|GetTargetingTeam (.MyStructure (Utilities|Struct|BreakPrimalSaddleStructure _array_element))) (Variables|Default|GetTargetingTeam)) (not (== (.MyStructure (Utilities|Struct|BreakPrimalSaddleStructure _array_element)) self)))
                      (bind _asprimalstructure (Utilities|Casting|CastToPrimalStructureClass (Utilities|GetClass (.MyStructure (Utilities|Struct|BreakPrimalSaddleStructure _array_element)))))
                      (if (Utilities|Array|ContainsItem (Variables|Default|GetdistributeForgeStructureWhitelist) _asprimalstructure)
                        (bind _asprimalstructureitemcontainer (Utilities|Casting|CastToPrimalStructureItemContainer (.MyStructure (Utilities|Struct|BreakPrimalSaddleStructure _array_element))))
                        (Utilities|Array|Add (LocalVariables|GetnearbyForgeInventories) (Variables|/Script/ShooterGame.PrimalStructureItemContainer|GetMyInventoryComponent _asprimalstructureitemcontainer))))))
                (:Is%20Not%20Valid
                  ;[1 1 1] Gets all forge structures in range
                  (for _array_element_2 (Variables|Default|GetdistributeForgeStructureWhitelist)
                    (bind _returnvalue_2 (Class|VictoryCore|ServerOctreeOverlapActorsClass (Class|Actor|GetWorld) (Transformation|GetActorLocation) (Variables|Default|GeteffectRange) "STRUCTURES" _array_element_2 false))
                    (for _array_element_3 _returnvalue_2
                      ;[1 1 1] Makes sure the forge structures are valid and gets a list of their inventories
                      (if (== (Variables|/Script/Engine.Actor|GetTargetingTeam _array_element_3) (Variables|Default|GetTargetingTeam))
                        (bind _asprimalstructureitemcontainer_2 (Utilities|Casting|CastToPrimalStructureItemContainer _array_element_3))
                        (Utilities|Array|Add (LocalVariables|GetnearbyForgeInventories) (Variables|/Script/ShooterGame.PrimalStructureItemContainer|GetMyInventoryComponent _asprimalstructureitemcontainer_2))))))))
            (:then_1
              ;[1 1 1] Gets all forge dinos in range
              (for _array_element_4 (Variables|Default|GetdistributeForgeDinoWhitelist)
                (bind _returnvalue_3 (Class|VictoryCore|ServerOctreeOverlapActorsClass (Class|Actor|GetWorld) (Transformation|GetActorLocation) (Variables|Default|GeteffectRange) "STRUCTURES" _array_element_4 false))
                (for _array_element_5 _returnvalue_3
                  ;[1 1 1] Makes sure the forge dinos are valid and gets a list of their inventories
                  (if (== (Variables|/Script/Engine.Actor|GetTargetingTeam _array_element_5) (Variables|Default|GetTargetingTeam))
                    (bind _asprimaldinocharacter (Utilities|Casting|CastToPrimalDinoCharacter _array_element_5))
                    (Utilities|Array|Add (LocalVariables|GetnearbyForgeInventories) (Variables|/Script/ShooterGame.PrimalCharacter|GetMyInventoryComponent _asprimaldinocharacter))))))
            (:then_2
              ;[1 1 1] Distributes items to nearby inventories
              (if (> _returnvalue 0)
                (LocalVariables|SetinventoriesToTransferTo _returnvalue)
                (Utilities|FlowControl|Sequence
                  (:then_0
                    ;[1 1 1] Distributes metal between all valid inventories
                    (if (Variables|Default|GetisDistributeMetalActive)
                      (bind _returnvalue_4 (Class|PrimalInventoryComponent|GetItemTemplateQuantity (Variables|Default|GetMyInventoryComponent) "/Game/PrimalEarth/CoreBlueprints/Resources/PrimalItemResource_Metal.PrimalItemResource_Metal_C" 0 true false false false))
                      (LocalVariables|SetamountToTransferWithoutRemainder (/ _returnvalue_4 (LocalVariables|GetinventoriesToTransferTo)))
                      (LocalVariables|SetamountToTransferRemainder (Math|Integer|%(Integer) _returnvalue_4 (LocalVariables|GetinventoriesToTransferTo)))
                      (if (or (> (LocalVariables|GetamountToTransferWithoutRemainder) 0) (> (LocalVariables|GetamountToTransferRemainder) 0))
                        (for _array_element_6 (LocalVariables|GetnearbyForgeInventories)
                          (if (> (LocalVariables|GetamountToTransferRemainder) 0)
                            (CallFunction|RUTransferItemQuantityfromInventory (Variables|Default|GetMyInventoryComponent) _array_element_6 "/Game/PrimalEarth/CoreBlueprints/Resources/PrimalItemResource_Metal.PrimalItemResource_Metal_C" (+ (LocalVariables|GetamountToTransferWithoutRemainder) 1) false false false false)
                            (LocalVariables|SetamountToTransferRemainder (- (LocalVariables|GetamountToTransferRemainder) 1))
                            (else
                              (CallFunction|RUTransferItemQuantityfromInventory (Variables|Default|GetMyInventoryComponent) _array_element_6 "/Game/PrimalEarth/CoreBlueprints/Resources/PrimalItemResource_Metal.PrimalItemResource_Metal_C" (LocalVariables|GetamountToTransferWithoutRemainder) false false false false)))))))
                  (:then_1
                    ;[1 1 1] Distributes wood between all valid inventories
                    (if (Variables|Default|GetisDistributeWoodActive)
                      (bind _returnvalue_5 (Class|PrimalInventoryComponent|GetItemTemplateQuantity (Variables|Default|GetMyInventoryComponent) "/Game/PrimalEarth/CoreBlueprints/Resources/PrimalItemResource_Wood.PrimalItemResource_Wood_C" 0 true false false false))
                      (LocalVariables|SetamountToTransferWithoutRemainder (/ _returnvalue_5 (LocalVariables|GetinventoriesToTransferTo)))
                      (LocalVariables|SetamountToTransferRemainder (Math|Integer|%(Integer) _returnvalue_5 (LocalVariables|GetinventoriesToTransferTo)))
                      (if (or (> (LocalVariables|GetamountToTransferWithoutRemainder) 0) (> (LocalVariables|GetamountToTransferRemainder) 0))
                        (for _array_element_7 (LocalVariables|GetnearbyForgeInventories)
                          (if (> (LocalVariables|GetamountToTransferRemainder) 0)
                            (CallFunction|RUTransferItemQuantityfromInventory (Variables|Default|GetMyInventoryComponent) _array_element_7 "/Game/PrimalEarth/CoreBlueprints/Resources/PrimalItemResource_Wood.PrimalItemResource_Wood_C" (+ (LocalVariables|GetamountToTransferWithoutRemainder) 1) false false false false)
                            (LocalVariables|SetamountToTransferRemainder (- (LocalVariables|GetamountToTransferRemainder) 1))
                            (else
                              (CallFunction|RUTransferItemQuantityfromInventory (Variables|Default|GetMyInventoryComponent) _array_element_7 "/Game/PrimalEarth/CoreBlueprints/Resources/PrimalItemResource_Wood.PrimalItemResource_Wood_C" (LocalVariables|GetamountToTransferWithoutRemainder) false false false false))))))))))))))))

(fn UnpackagePallets
  (bind _myinventorycomponent (Variables|Default|GetMyInventoryComponent))
  (LocalVariables|SetinventoryItemsAtStart (Variables|/Script/ShooterGame.PrimalInventoryComponent|GetInventoryItems (Variables|Default|GetMyInventoryComponent)))
  ;[1 1 1] Loops through all items in the packager, only trying to unpack the pallets that aren't blueprints
  (bind _array_element (Utilities|Array|ForEachLoopwithBreak (LocalVariables|GetinventoryItemsAtStart) :!label _label)
    (:LoopBody
      (if (LocalVariables|GetisInventoryFull)
        (goto _label Break)
        (elif (and (not (Variables|/Script/ShooterGame.PrimalItem|GetbIsBlueprint _array_element)) (Class|VictoryCore|ObjectIsChildOf _array_element "/Game/Mods/RosesUtilities/Items/Resources/Pallets/PrimalItemResourcePallet_Base.PrimalItemResourcePallet_Base_C" false))
          ;[1 1 1] Unpacks pallets 1 quantity at a time
          (LocalVariables|SetpalletQuantity (Variables|/Script/ShooterGame.PrimalItem|GetItemQuantity _array_element))
          (Utilities|FlowControl|ForLoopwithBreak 1 (LocalVariables|GetpalletQuantity) :!label _label_2
            (:LoopBody
              ;[1 1 1] Prevents and halts unpackaging if there isn't enough room for the items from the pallet
              (if (< (- (Utilities|Array|Length (Variables|/Script/ShooterGame.PrimalInventoryComponent|GetInventoryItems _myinventorycomponent)) 15) (Variables|/Script/ShooterGame.PrimalInventoryComponent|GetAbsoluteMaxInventoryItems _myinventorycomponent))
                ;[1 1 1] Adds the contents of the pallet and then removes one instance of the pallet
                (Class|PrimalInventoryComponent|BPIncrementItemTemplateQuantity (Variables|Default|GetMyInventoryComponent) (.ResourceItemType (Utilities|Struct|BreakCraftingResourceRequirement (Utilities|Array|Get(acopy) (Variables|/Script/ShooterGame.PrimalItem|GetBaseCraftingResourceRequirements _array_element)))) (Math|Float|Floor (.BaseResourceRequirement (Utilities|Struct|BreakCraftingResourceRequirement (Utilities|Array|Get(acopy) (Variables|/Script/ShooterGame.PrimalItem|GetBaseCraftingResourceRequirements _array_element))))) true false true false false false 0 false)
                (bind _asprimalitem (Utilities|Casting|CastToPrimalItemClass (Utilities|GetClass _array_element)))
                (Class|PrimalInventoryComponent|BPIncrementItemTemplateQuantity (Variables|Default|GetMyInventoryComponent) _asprimalitem -1 true false true false false false 0 false)
                (else
                  (LocalVariables|SetisInventoryFull true)
                  (goto _label_2 Break))))))))))

(fn OnRepIsDistributeWoodActive
  ;[1 1 1] Disables the auto-crafting of each wood pallet type
  (bind _array_element (Utilities|Array|ForEachLoopwithBreak (Variables|/Script/ShooterGame.PrimalInventoryComponent|GetInventoryItems (Variables|Default|GetMyInventoryComponent)) :!label _label)
    (:LoopBody
      (if (and (Variables|/Script/ShooterGame.PrimalItem|GetbIsBlueprint _array_element) (Math|Boolean|ORBoolean (== (Utilities|GetClass _array_element) "/Game/Mods/RosesUtilities/Items/Resources/Pallets/PrimalItemResourcePallet_Wood.PrimalItemResourcePallet_Wood_C") (== (Utilities|GetClass _array_element) "/Game/Mods/RosesUtilities/Items/Resources/Pallets/PrimalItemResourcePallet_FungalWood.PrimalItemResourcePallet_FungalWood_C") (== (Utilities|GetClass _array_element) "/Game/Mods/RosesUtilities/Items/Resources/Pallets/PrimalItemResourcePallet_CorruptedWood.PrimalItemResourcePallet_CorruptedWood_C")))
        (Variables|/Script/ShooterGame.PrimalItem|SetbAutoCraftBlueprint _array_element (not (Variables|Default|GetisDistributeWoodActive)))
        (Class|PrimalItem|UpdatedItem _array_element false)
        ;[1 1 1] Marks that type of wood pallet as enabled or disabled so once all 3 are in the correct state, it can stop looping
        (if (== (Utilities|GetClass _array_element) "/Game/Mods/RosesUtilities/Items/Resources/Pallets/PrimalItemResourcePallet_Wood.PrimalItemResourcePallet_Wood_C")
          (LocalVariables|SetisWoodDisabled true)
          (if (Math|Boolean|ANDBoolean (LocalVariables|GetisWoodDisabled) (LocalVariables|GetisFungalDisabled) (LocalVariables|GetisCorruptedDisabled)) :!label _label_2
            (goto _label Break))
          (elif (== (Utilities|GetClass _array_element) "/Game/Mods/RosesUtilities/Items/Resources/Pallets/PrimalItemResourcePallet_FungalWood.PrimalItemResourcePallet_FungalWood_C")
            (LocalVariables|SetisFungalDisabled true)
            (goto _label_2)
            (elif (== (Utilities|GetClass _array_element) "/Game/Mods/RosesUtilities/Items/Resources/Pallets/PrimalItemResourcePallet_CorruptedWood.PrimalItemResourcePallet_CorruptedWood_C")
              (LocalVariables|SetisCorruptedDisabled true)
              (goto _label_2))))))))