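; Communal nest structure that auto-collects team eggs dropped in range, incubates fertilized ones in its inventory and toggles mating on nearby tames.
; Server timers drive collection, incubation and optional mating shutoff when full, using global config and hatch-speed settings.
; The radial menu offers a species filter from nearby dinos, resolving egg classes through a temporarily spawned dino.
; Unfiltered nests skip species claimed by nearby filtered nests and Dino Daycares.
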(event Custom|GetFilter
  ;[1 1 1] Event allows restricting getting the filter options to once every 5 seconds
  (if (not (Variables|Default|GetfilterCheckLocked))
    (CallFunction|GetFilterOptions)
    (Utilities|FlowControl|Delay 5.0)
    (Variables|Default|SetfilterCheckLocked false)))

(event Custom|OpenFilterSubMenu
  (params (playerController :type Player%20Controller%20Object%20Reference))
  (CallFunction|BPClientDoMultiUse playerController 90515))

(event EventParentFirstBeginPlay
  (Utilities|FlowControl|Sequence
    (:then_0
      ;[1 1 1] Gets auto-collect range config
      (Class|KismetSystemLibrary|IsRunningonServer
        (:Yes
          (bind _globalactor (CallFunction|RUGetGlobalActor self))
          (Variables|Default|SeteffectRange (* 300 (Variables|/Game/Mods/RosesUtilities/RosesUtilities_GlobalActor.RosesUtilities_GlobalActor_C|GetCommunalNestAutoCollectRange _globalactor)) true)
          ;[1 1 1] Gets incubation rate config
          (Variables|Default|SetincubationMultiplier (Variables|/Game/Mods/RosesUtilities/RosesUtilities_GlobalActor.RosesUtilities_GlobalActor_C|GetCommunalNestIncubationRate _globalactor) true)
          ;[1 1 1] Gets disable mating when full config
          (Variables|Default|SetshouldDisableMatingWhenFull (Variables|/Game/Mods/RosesUtilities/RosesUtilities_GlobalActor.RosesUtilities_GlobalActor_C|GetCommunalNestDisableMatingWhenFull _globalactor) true)
          ;[1 1 1] Gets hatch speed from server config
          (bind _asshootergamestate (Utilities|Casting|CastToShooterGameState (Game|GetGameState)))
          (Variables|Default|SetserverEggHatchSpeedMultiplier (Variables|/Script/ShooterGame.ShooterGameState|GetEggHatchSpeedMultiplier _asshootergamestate)))))
    (:then_1
      ;[1 1 1] Restores saved visibility
      (CallFunction|OnRepEffectRange))
    (:then_2
      ;[1 1 1] Starts collect item scan, incubate eggs loops, and disable mating when full check
      (Class|KismetSystemLibrary|IsRunningonServer
        (:Yes
          (Utilities|FlowControl|Delay 0.5)
          (Utilities|Time|SetTimerbyFunctionName 0 "AutoCollectItems" 1e+01 true)
          (Utilities|FlowControl|Delay 1.0)
          (Utilities|Time|SetTimerbyFunctionName 0 "IncubateEggs" 1e+01 true)
          (if (Variables|Default|GetshouldDisableMatingWhenFull)
            (Utilities|FlowControl|Delay 1.0)
            (Utilities|Time|SetTimerbyFunctionName 0 "DisableMatingWhenFull" 6e+01 true)))))))

(fn ConstructionScript
  (|CallParentFunction))

(fn BPGetMultiUseEntries
  (params (ForPC :type Player%20Controller%20Object%20Reference) (MultiUseEntries :type Array%20of%20Multi%20Use%20Entry%20Structures))
  (bind _isautocollectactive_fertilized (Variables|Default|GetisAutoCollectActive_Fertilized))
  (bind _isautocollectactive_unfertilized (Variables|Default|GetisAutoCollectActive_Unfertilized))
  (bind _dinofilteroptions (Variables|Default|GetdinoFilterOptions))
  (bind _dinofilteroptions_2 (Variables|Default|GetdinoFilterOptions))
  (bind _dinofilteroptions_3 (Variables|Default|GetdinoFilterOptions))
  (bind _dinofilteroptions_4 (Variables|Default|GetdinoFilterOptions))
  (bind _dinofilteroptions_5 (Variables|Default|GetdinoFilterOptions))
  (bind _returnvalue (|CallParentFunction ForPC MultiUseEntries))
  (LocalVariables|SettempMultiUseEntries _returnvalue)
  (if (== (Variables|Default|GetTargetingTeam) (Variables|/Script/Engine.Actor|GetTargetingTeam ForPC))
    (CallFunction|GetFilter)
    (Utilities|FlowControl|Sequence
      (:then_0
        (Utilities|FlowControl|Sequence
          (:then_0
            ;[1 1 1] Adds a MultiUse entry to toggle auto collecting unfertilized eggs on or off
            (Utilities|Array|Add (LocalVariables|GettempMultiUseEntries) (Utilities|Struct|MakeMultiUseEntry 0 (Utilities|String|SelectString "Auto-Collect Unfertilized Eggs [Enabled]" "Auto-Collect Unfertilized Eggs [Disabled]" _isautocollectactive_unfertilized) 90314 -9999 false false false false false false false false false true false false false false 0 "(B=175,G=175,R=175,A=255)" (Math|Conversions|ToColor(LinearColor) (Math|Color|SelectColor "(R=0.250000,G=1.000000,B=0.250000,A=1.000000)" "(R=1.000000,G=0.250000,B=0.250000,A=1.000000)" _isautocollectactive_unfertilized)))))
          (:then_1
            ;[1 1 1] Adds a MultiUse entry to toggle auto collecting fertilized eggs on or off
            (Utilities|Array|Add (LocalVariables|GettempMultiUseEntries) (Utilities|Struct|MakeMultiUseEntry 0 (Utilities|String|SelectString "Auto-Collect Fertilized Eggs [Enabled]" "Auto-Collect Fertilized Eggs [Disabled]" _isautocollectactive_fertilized) 90414 -10000 false false false false false false false false false true false false false false 0 "(B=175,G=175,R=175,A=255)" (Math|Conversions|ToColor(LinearColor) (Math|Color|SelectColor "(R=0.250000,G=1.000000,B=0.250000,A=1.000000)" "(R=1.000000,G=0.250000,B=0.250000,A=1.000000)" _isautocollectactive_fertilized)))))
          (:then_2
            ;[1 1 1] Adds a MultiUse entry to enable mating for nearby dinos (all or the current filter if valid)
            (bind _descriptivename (CallFunction|RUGetDescriptiveName (Variables|Default|GetdinoFilter)))
            (bind _isfilterset (CallFunction|IsDinoFilterSet))
            (Utilities|Array|Add (LocalVariables|GettempMultiUseEntries) (Utilities|Struct|MakeMultiUseEntry 0 (Utilities|String|SelectString "Enable Nearby Mating" (Utilities|String|JoinStringArray (Utilities|Array|MakeArray "Enable Nearby Mating {" _descriptivename ")") "") (not _isfilterset)) 90520 -9001 false false false false false false false false false true false false false false 0 "(B=175,G=175,R=175,A=255)" (Math|Conversions|ToColor(LinearColor) (Math|Color|SelectColor "(R=0.250000,G=1.000000,B=0.250000,A=1.000000)" "(R=1.000000,G=0.250000,B=0.250000,A=1.000000)" true)))))
          (:then_3
            ;[1 1 1] Adds a MultiUse entry to disable mating for nearby dinos (all or the current filter if valid)
            (bind _descriptivename_2 (CallFunction|RUGetDescriptiveName (Variables|Default|GetdinoFilter)))
            (bind _isfilterset_2 (CallFunction|IsDinoFilterSet))
            (Utilities|Array|Add (LocalVariables|GettempMultiUseEntries) (Utilities|Struct|MakeMultiUseEntry 0 (Utilities|String|SelectString "Disable Nearby Mating" (Utilities|String|JoinStringArray (Utilities|Array|MakeArray "Disable Nearby Mating {" _descriptivename_2 ")") "") (not _isfilterset_2)) 90521 -9000 false false false false false false false false false true false false false false 0 "(B=175,G=175,R=175,A=255)" (Math|Conversions|ToColor(LinearColor) (Math|Color|SelectColor "(R=0.250000,G=1.000000,B=0.250000,A=1.000000)" "(R=1.000000,G=0.250000,B=0.250000,A=1.000000)" false)))))))
      (:then_1
        (Utilities|FlowControl|Sequence
          (:then_0
            ;[1 1 1] Adds a MultiUse entry to open the dino filter menu or reset the filter if valid
            (bind _descriptivename_3 (CallFunction|RUGetDescriptiveName (Variables|Default|GetdinoFilter)))
            (bind _isfilterset_3 (CallFunction|IsDinoFilterSet))
            (Utilities|Array|Add (LocalVariables|GettempMultiUseEntries) (Utilities|Struct|MakeMultiUseEntry 0 (Utilities|String|SelectString "Create Egg Filter" (Utilities|String|JoinStringArray (Utilities|Array|MakeArray "Remove Egg Filter (" _descriptivename_3 ")") "") (not _isfilterset_3)) 90514 -10002 false false false false false false false false true true false false false false 0 "(B=175,G=175,R=175,A=255)" (Math|Color|MakeColor 255 200 255 255))))
          (:then_1
            ;[1 1 1] Adds a MultiUse entry Back option to create filter menu
            (Utilities|Array|Add (LocalVariables|GettempMultiUseEntries) (Utilities|Struct|MakeMultiUseEntry 0 "[Back]" 91501 0 false false false false false false false false true true false false false false 91500 "(B=175,G=175,R=175,A=255)" (Math|Color|MakeColor 200 255 100 255))))
          (:then_2
            ;[1 1 1] Adds a MultiUse entry for the 1st filter option
            (if (>= (Utilities|Array|Length _dinofilteroptions_2) 1)
              (bind _descriptivename_4 (CallFunction|RUGetDescriptiveName (Utilities|Array|Get(acopy) _dinofilteroptions_2)))
              (Utilities|Array|Add (LocalVariables|GettempMultiUseEntries) (Utilities|Struct|MakeMultiUseEntry 0 _descriptivename_4 91502 -5 false false false false false false false false true false false false false false 91500 "(B=175,G=175,R=175,A=255)" (Math|Color|MakeColor 255 200 255 255)))))
          (:then_3
            ;[1 1 1] Adds a MultiUse entry for the 2nd filter option
            (if (>= (Utilities|Array|Length _dinofilteroptions_3) 2)
              (bind _descriptivename_5 (CallFunction|RUGetDescriptiveName (Utilities|Array|Get(acopy) _dinofilteroptions_3 1)))
              (Utilities|Array|Add (LocalVariables|GettempMultiUseEntries) (Utilities|Struct|MakeMultiUseEntry 0 _descriptivename_5 91503 -4 false false false false false false false false true false false false false false 91500 "(B=175,G=175,R=175,A=255)" (Math|Color|MakeColor 255 200 255 255)))))
          (:then_4
            ;[1 1 1] Adds a MultiUse entry for the 3rd filter option
            (if (>= (Utilities|Array|Length _dinofilteroptions_4) 3)
              (bind _descriptivename_6 (CallFunction|RUGetDescriptiveName (Utilities|Array|Get(acopy) _dinofilteroptions_4 2)))
              (Utilities|Array|Add (LocalVariables|GettempMultiUseEntries) (Utilities|Struct|MakeMultiUseEntry 0 _descriptivename_6 91504 -3 false false false false false false false false true false false false false false 91500 "(B=175,G=175,R=175,A=255)" (Math|Color|MakeColor 255 200 255 255)))))
          (:then_5
            ;[1 1 1] Adds a MultiUse entry for the 4th filter option
            (if (>= (Utilities|Array|Length _dinofilteroptions_5) 4)
              (bind _descriptivename_7 (CallFunction|RUGetDescriptiveName (Utilities|Array|Get(acopy) _dinofilteroptions_5 3)))
              (Utilities|Array|Add (LocalVariables|GettempMultiUseEntries) (Utilities|Struct|MakeMultiUseEntry 0 _descriptivename_7 91505 -2 false false false false false false false false true false false false false false 91500 "(B=175,G=175,R=175,A=255)" (Math|Color|MakeColor 255 200 255 255)))))
          (:then_6
            ;[1 1 1] Adds a MultiUse entry for the 5th filter option
            (if (>= (Utilities|Array|Length _dinofilteroptions) 5)
              (bind _descriptivename_8 (CallFunction|RUGetDescriptiveName (Utilities|Array|Get(acopy) _dinofilteroptions 4)))
              (Utilities|Array|Add (LocalVariables|GettempMultiUseEntries) (Utilities|Struct|MakeMultiUseEntry 0 _descriptivename_8 91506 -1 false false false false false false false false true false false false false false 91500 "(B=175,G=175,R=175,A=255)" (Math|Color|MakeColor 255 200 255 255)))))))
      (:then_2
        (return (LocalVariables|GettempMultiUseEntries))))
    (else
      (return (LocalVariables|GettempMultiUseEntries)))))

(fn BPTryMultiUse
  (params (ForPC :type Player%20Controller%20Object%20Reference) (UseIndex :type Integer))
  (bind _returnvalue (Utilities|String|ToString(Integer) UseIndex))
  (bind _dinofilteroptions (Variables|Default|GetdinoFilterOptions))
  (bind _dinofilteroptions_2 (Variables|Default|GetdinoFilterOptions))
  (bind _dinofilteroptions_3 (Variables|Default|GetdinoFilterOptions))
  (bind _dinofilteroptions_4 (Variables|Default|GetdinoFilterOptions))
  (bind _dinofilteroptions_5 (Variables|Default|GetdinoFilterOptions))
  (bind _item (Utilities|Array|Get(acopy) _dinofilteroptions 4))
  (bind _item_2 (Utilities|Array|Get(acopy) _dinofilteroptions_5))
  (bind _item_3 (Utilities|Array|Get(acopy) _dinofilteroptions_2 1))
  (bind _item_4 (Utilities|Array|Get(acopy) _dinofilteroptions_3 2))
  (bind _item_5 (Utilities|Array|Get(acopy) _dinofilteroptions_4 3))
  (|CallParentFunction ForPC UseIndex)
  (LocalVariables|SetplayerController ForPC)
  (Utilities|FlowControl|Sequence
    (:then_0
      (switch string _returnvalue
        (:Default
          (switch string _returnvalue
            (:90514
              ;[1 1 1] Opens dino filter menu or resets filter
              (bind _isfilterset (CallFunction|IsDinoFilterSet))
              (if (not _isfilterset)
                ;[1 1 1] Opens the filter selection menu if there are dinos to add to the filter
                (if (>= (Utilities|Array|Length (Variables|Default|GetdinoFilterOptions)) 1)
                  (bind _asshooterplayercontroller (Utilities|Casting|CastToShooterPlayerController (LocalVariables|GetplayerController)))
                  (CallFunction|OpenFilterSubMenu _asshooterplayercontroller)
                  (else
                    ;[1 1 1] Warns if there are no nearby dinos to be filter options
                    (CallFunction|RUMessageClient (LocalVariables|GetplayerController) "No nearby valid dinos to create filter from!" "NewEnumerator1")))
                (else
                  ;[1 1 1] Resets dino filter
                  (Variables|Default|SetdinoFilter "/Script/ShooterGame.PrimalDinoCharacter" true)
                  (CallFunction|RUMessageClient (LocalVariables|GetplayerController) "Communal Nest picking up all eggs" "NewEnumerator2"))))
            (:91502
              ;[1 1 1] Sets dino filter to 1st filter selection
              (if (>= (Utilities|Array|Length _dinofilteroptions_5) 1)
                (Variables|Default|SetdinoFilter _item_2 true)
                (bind _descriptivename (CallFunction|RUGetDescriptiveName _item_2))
                (CallFunction|RUMessageClient (LocalVariables|GetplayerController) (Utilities|String|JoinStringArray (Utilities|Array|MakeArray "Communal Nest picking up " _descriptivename " eggs") "") "NewEnumerator2")
                ;[1 1 1] Gets Fertilized and Unfertilized egg classes to filter by
                (bind _returnvalue_2 (Class|ShooterGameViewportClient|GetGameWorld :!label _label))
                (bind _returnvalue_3 (Class|PrimalDinoCharacter|SpawnDino _returnvalue_2 (Variables|Default|GetdinoFilter) "0,0.000000, 0" "0, 0, 0" 1.0 0 false false 0 false 1.0 0 false))
                (Variables|Default|SetdinoFilterEggs (Variables|/Script/ShooterGame.PrimalDinoCharacter|GetFertilizedEggItemsToSpawn _returnvalue_3))
                (Utilities|Array|AppendArray (Variables|Default|GetdinoFilterEggs) (Variables|/Script/ShooterGame.PrimalDinoCharacter|GetEggItemsToSpawn _returnvalue_3))
                (if (Utilities|ClassIsChildOf (Variables|Default|GetdinoFilter) "/Game/PrimalEarth/Dinos/Dodo/Dodo_Character_BP.Dodo_Character_BP_C")
                  (Utilities|Array|Add (Variables|Default|GetdinoFilterEggs) (Variables|/Script/ShooterGame.PrimalCharacter|GetPoopAltItemClass _returnvalue_3)))
                (Actor|DestroyActor _returnvalue_3)))
            (:91503
              ;[1 1 1] Sets dino filter to 2nd filter selection
              (if (>= (Utilities|Array|Length _dinofilteroptions_2) 2)
                (Variables|Default|SetdinoFilter _item_3 true)
                (bind _descriptivename_2 (CallFunction|RUGetDescriptiveName _item_3))
                (CallFunction|RUMessageClient (LocalVariables|GetplayerController) (Utilities|String|JoinStringArray (Utilities|Array|MakeArray "Communal Nest picking up " _descriptivename_2 " eggs") "") "NewEnumerator2")
                (goto _label)))
            (:91504
              ;[1 1 1] Sets dino filter to 3rd filter selection
              (if (>= (Utilities|Array|Length _dinofilteroptions_3) 3)
                (Variables|Default|SetdinoFilter _item_4 true)
                (bind _descriptivename_3 (CallFunction|RUGetDescriptiveName _item_4))
                (CallFunction|RUMessageClient (LocalVariables|GetplayerController) (Utilities|String|JoinStringArray (Utilities|Array|MakeArray "Communal Nest picking up " _descriptivename_3 " eggs") "") "NewEnumerator2")
                (goto _label)))
            (:91505
              ;[1 1 1] Sets dino filter to 4th filter selection
              (if (>= (Utilities|Array|Length _dinofilteroptions_4) 4)
                (Variables|Default|SetdinoFilter _item_5 true)
                (bind _descriptivename_4 (CallFunction|RUGetDescriptiveName _item_5))
                (CallFunction|RUMessageClient (LocalVariables|GetplayerController) (Utilities|String|JoinStringArray (Utilities|Array|MakeArray "Communal Nest picking up " _descriptivename_4 " eggs") "") "NewEnumerator2")
                (goto _label)))
            (:91506
              ;[1 1 1] Sets dino filter to 5th filter selection
              (if (>= (Utilities|Array|Length _dinofilteroptions) 5)
                (Variables|Default|SetdinoFilter _item true)
                (bind _descriptivename_5 (CallFunction|RUGetDescriptiveName _item))
                (CallFunction|RUMessageClient (LocalVariables|GetplayerController) (Utilities|String|JoinStringArray (Utilities|Array|MakeArray "Communal Nest picking up " _descriptivename_5 " eggs") "") "NewEnumerator2")
                (goto _label)))))
        (:90314
          ;[1 1 1] Toggles unfertilized auto-collect
          (Variables|Default|SetisAutoCollectActive_Unfertilized (not (Variables|Default|GetisAutoCollectActive_Unfertilized)) true))
        (:90414
          ;[1 1 1] Toggles fertilized auto-collect
          (Variables|Default|SetisAutoCollectActive_Fertilized (not (Variables|Default|GetisAutoCollectActive_Fertilized)) true))
        (:90520
          ;[1 1 1] Enables mating in radius
          (CallFunction|ToggleMatinginRadius true)
          (CallFunction|RUMessageClient (LocalVariables|GetplayerController) "Mating enabled for nearby dinos!" "NewEnumerator2"))
        (:90521
          ;[1 1 1] Disables mating in radius
          (CallFunction|ToggleMatinginRadius false)
          (CallFunction|RUMessageClient (LocalVariables|GetplayerController) "Mating disabled for nearby dinos!" "NewEnumerator2"))))
    (:then_1
      (return true))))

(fn AutoCollectItems
  (Class|KismetSystemLibrary|IsRunningonServer
    (:Yes
      ;[1 1 1] Disables if range is 0
      (if (> (Variables|Default|GeteffectRange) 0.0)
        ;[1 1 1] Cancels collection if neither egg type is enabled
        (if (or (Variables|Default|GetisAutoCollectActive_Fertilized) (Variables|Default|GetisAutoCollectActive_Unfertilized))
          (Utilities|FlowControl|Sequence
            (:then_0
              ;[1 1 1] If the filter is unset, gets the egg filters of nearby Dino Daycares and Communal Nests to prevent affecting their eggs
              (bind _isfilterset (CallFunction|IsDinoFilterSet))
              (if (not _isfilterset)
                (Utilities|FlowControl|Sequence
                  (:then_0
                    (bind _returnvalue (Class|VictoryCore|ServerOctreeOverlapActorsClass (Class|Actor|GetWorld) (Transformation|GetActorLocation) (Variables|Default|GeteffectRange) "STRUCTURES" "/Game/Mods/RosesUtilities/Structures/DinoDaycare/BP_DinoDaycare.BP_DinoDaycare_C" false))
                    (for _array_element _returnvalue
                      (bind _asbp_dinodaycare_c (Utilities|Casting|CastToBP_DinoDaycare _array_element))
                      (bind _isfilterset_2 (Default|IsDinoFilterSet _asbp_dinodaycare_c))
                      (if _isfilterset_2
                        (for _array_element_2 (Variables|/Game/Mods/RosesUtilities/Structures/DinoDaycare/BP_DinoDaycare.BP_DinoDaycare_C|GetdinoFilterEggs _asbp_dinodaycare_c)
                          (Utilities|Array|AddUnique (LocalVariables|GetdinoEggClassesToIgnore) _array_element_2)))))
                  (:then_1
                    (bind _returnvalue_2 (Class|VictoryCore|ServerOctreeOverlapActorsClass (Class|Actor|GetWorld) (Transformation|GetActorLocation) (Variables|Default|GeteffectRange) "STRUCTURES" "BP_CommunalNest_C" false))
                    (for _array_element_3 _returnvalue_2
                      (bind _asbp_communalnest_c (Utilities|Casting|CastToBP_CommunalNest _array_element_3))
                      (bind _isfilterset_3 (CallFunction|IsDinoFilterSet _asbp_communalnest_c))
                      (if _isfilterset_3
                        (for _array_element_4 (Variables|BP_CommunalNest_C|GetdinoFilterEggs _asbp_communalnest_c)
                          (Utilities|Array|AddUnique (LocalVariables|GetdinoEggClassesToIgnore) _array_element_4))))))))
            (:then_1
              ;[1 1 1] Gets all dropped items in range
              (bind _returnvalue_3 (Class|VictoryCore|ServerOctreeOverlapActorsClass (Class|Actor|GetWorld) (Transformation|GetActorLocation) (Variables|Default|GeteffectRange) "ALL_SPATIAL" "/Script/ShooterGame.DroppedItem" true))
              ;[1 1 1] Picks up each dropped egg in range
              (for _array_element_5 _returnvalue_3
                (if (== (Variables|/Script/Engine.Actor|GetTargetingTeam _array_element_5) (Variables|Default|GetTargetingTeam))
                  (bind _asdroppeditem (Utilities|Casting|CastToDroppedItem _array_element_5))
                  ;[1 1 1] Filters pickup based on if Fertilized or/and Unfertilized should be picked up
                  (bind _asprimalitemconsumable_egg_c (Utilities|Casting|CastToPrimalItemConsumable_Egg (Variables|/Script/ShooterGame.DroppedItem|GetMyItem _asdroppeditem)))
                  (bind _isfertilized (CallFunction|RUIsEggFertilized _asprimalitemconsumable_egg_c))
                  (if (Math|Boolean|ORBoolean (Math|Boolean|ANDBoolean (Variables|Default|GetisAutoCollectActive_Fertilized) (not (Variables|Default|GetisAutoCollectActive_Unfertilized)) _isfertilized) (Math|Boolean|ANDBoolean (not (Variables|Default|GetisAutoCollectActive_Fertilized)) (Variables|Default|GetisAutoCollectActive_Unfertilized) (not _isfertilized)) (and (Variables|Default|GetisAutoCollectActive_Fertilized) (Variables|Default|GetisAutoCollectActive_Unfertilized)))
                    ;[1 1 1] If filter is active, only picks up matching eggs, otherwise avoids picking up eggs filtered by other structures nearby
                    (bind _asprimalitem (Utilities|Casting|CastToPrimalItemClass (Utilities|GetClass _asprimalitemconsumable_egg_c)))
                    (bind _isfilterset_4 (CallFunction|IsDinoFilterSet))
                    (if (or (and _isfilterset_4 (Utilities|Array|ContainsItem (Variables|Default|GetdinoFilterEggs) _asprimalitem)) (and (not _isfilterset_4) (not (Utilities|Array|ContainsItem (LocalVariables|GetdinoEggClassesToIgnore) _asprimalitem))))
                      ;[1 1 1] Prevents picking up eggs that are done incubating
                      (bind _isfertilized_2 (CallFunction|RUIsEggFertilized _asprimalitemconsumable_egg_c))
                      (if _isfertilized_2
                        (if (> (Variables|/Script/ShooterGame.PrimalItem|GetItemDurability _asprimalitemconsumable_egg_c) 3.0)
                          (Utilities|FlowControl|Sequence :!label _label
                            (:then_0
                              ;[1 1 1] Stasis check
                              (if (Variables|/Script/Engine.Actor|GetbStasised _asdroppeditem)
                                (Class|Actor|Unstasis _asdroppeditem)))
                            (:then_1
                              ;[1 1 1] Adds egg to inventory and destroys dropped item actor
                              (CallFunction|RUPickupItemtoInventory _asdroppeditem (Variables|Default|GetMyInventoryComponent) (Utilities|Array|MakeArray "/Game/PrimalEarth/CoreBlueprints/Items/Consumables/PrimalItemConsumable_Egg.PrimalItemConsumable_Egg_C")))))
                        (else
                          (goto _label))))))))))))))

(fn IncubateEggs
  (Networking|SwitchHasAuthority
    (:Authority
      ;[1 1 1] Gets each fertilized egg to incubate
      (for _array_element (Variables|/Script/ShooterGame.PrimalInventoryComponent|GetInventoryItems (Variables|Default|GetMyInventoryComponent))
        (bind _asprimalitemconsumable_egg_c (Utilities|Casting|CastToPrimalItemConsumable_Egg _array_element))
        (bind _isfertilized (CallFunction|RUIsEggFertilized _asprimalitemconsumable_egg_c))
        (if _isfertilized
          (LocalVariables|SeteggToIncubate _asprimalitemconsumable_egg_c)
          ;[1 1 1] Updates egg incubation
          (if (> (Variables|/Script/ShooterGame.PrimalItem|GetItemDurability (LocalVariables|GeteggToIncubate)) 1.0)
            (Variables|/Script/ShooterGame.PrimalItem|SetItemDurability (LocalVariables|GeteggToIncubate) (Math|Float|Clamp(Float) (- (Variables|/Script/ShooterGame.PrimalItem|GetItemDurability (LocalVariables|GeteggToIncubate)) (* 1e+01 (Variables|/Script/ShooterGame.PrimalItem|GetEggLoseDurabilityPerSecond (LocalVariables|GeteggToIncubate)) (Variables|/Script/ShooterGame.PrimalItem|GetExtraEggLoseDurabilityPerSecondMultiplier (LocalVariables|GeteggToIncubate)) (Variables|Default|GetincubationMultiplier) (Variables|Default|GetserverEggHatchSpeedMultiplier))) 1.0 1e+02))
            (Class|PrimalItem|UpdatedItem (LocalVariables|GeteggToIncubate) false)))))))

(fn OnRepIncubationMultiplier)

(fn DisableMatingwhenFull
  (Class|KismetSystemLibrary|IsRunningonServer
    (:Yes
      ;[1 1 1] Disables if range is 0
      (if (> (Variables|Default|GeteffectRange) 0.0)
        ;[1 1 1] Only disable mating if inventory is full
        (bind _hasemptyslots (CallFunction|RUDoesInventoryHaveEmptySlots (Variables|Default|GetMyInventoryComponent)))
        (if (not _hasemptyslots)
          ;[1 1 1] Toggles mating off in radius
          (if (Variables|Default|GetshouldDisableMatingWhenFull)
            (CallFunction|ToggleMatinginRadius false)))))))

(fn ToggleMatinginRadius
  (params (enableMating :type Boolean))
  (Class|KismetSystemLibrary|IsRunningonServer
    (:Yes
      ;[1 1 1] Disables if range is 0
      (if (> (Variables|Default|GeteffectRange) 0.0)
        (Utilities|FlowControl|Sequence
          (:then_0
            ;[1 1 1] If the filter is unset, gets the filters of nearby Dino Daycares and Communal Nests to prevent affecting their dinos
            (bind _isfilterset (CallFunction|IsDinoFilterSet))
            (if (not _isfilterset)
              (Utilities|FlowControl|Sequence
                (:then_0
                  (bind _returnvalue (Class|VictoryCore|ServerOctreeOverlapActorsClass (Class|Actor|GetWorld) (Transformation|GetActorLocation) (Variables|Default|GeteffectRange) "STRUCTURES" "/Game/Mods/RosesUtilities/Structures/DinoDaycare/BP_DinoDaycare.BP_DinoDaycare_C" false))
                  (for _array_element _returnvalue
                    (bind _asbp_dinodaycare_c (Utilities|Casting|CastToBP_DinoDaycare _array_element))
                    (bind _isfilterset_2 (Default|IsDinoFilterSet _asbp_dinodaycare_c))
                    (if _isfilterset_2
                      (Utilities|Array|AddUnique (LocalVariables|GetdinoClassesToIgnore) (Variables|/Game/Mods/RosesUtilities/Structures/DinoDaycare/BP_DinoDaycare.BP_DinoDaycare_C|GetdinoFilter _asbp_dinodaycare_c)))))
                (:then_1
                  (bind _returnvalue_2 (Class|VictoryCore|ServerOctreeOverlapActorsClass (Class|Actor|GetWorld) (Transformation|GetActorLocation) (Variables|Default|GeteffectRange) "STRUCTURES" "BP_CommunalNest_C" false))
                  (for _array_element_2 _returnvalue_2
                    (bind _asbp_communalnest_c (Utilities|Casting|CastToBP_CommunalNest _array_element_2))
                    (bind _isfilterset_3 (CallFunction|IsDinoFilterSet _asbp_communalnest_c))
                    (if _isfilterset_3
                      (Utilities|Array|AddUnique (LocalVariables|GetdinoClassesToIgnore) (Variables|BP_CommunalNest_C|GetdinoFilter _asbp_communalnest_c))))))))
          (:then_1
            ;[1 1 1] Gets all dinos in range
            (bind _returnvalue_3 (Class|VictoryCore|ServerOctreeOverlapActorsClass (Class|Actor|GetWorld) (Transformation|GetActorLocation) (Variables|Default|GeteffectRange) "DINOPAWNS_TAMED" (Variables|Default|GetdinoFilter) false))
            ;[1 1 1] Only affects owned dinos that don't match nearby Dino Daycare and Communal Nest filters
            (for _array_element_3 _returnvalue_3
              (if (== (Variables|/Script/Engine.Actor|GetTargetingTeam _array_element_3) (Variables|Default|GetTargetingTeam))
                (bind _isfilterset_4 (CallFunction|IsDinoFilterSet))
                (if _isfilterset_4
                  (bind _asprimaldinocharacter (Utilities|Casting|CastToPrimalDinoCharacter _array_element_3 :!label _label))
                  (LocalVariables|SettempDino _asprimaldinocharacter)
                  ;[1 1 1] Toggles mating for dino
                  (Utilities|FlowControl|Sequence
                    (:then_0
                      ;;[1 1 1] Stasis check
                      (if (Variables|/Script/Engine.Actor|GetbStasised (LocalVariables|GettempDino))
                        (Class|Actor|Unstasis (LocalVariables|GettempDino))))
                    (:then_1
                      (Variables|/Script/ShooterGame.PrimalDinoCharacter|SetbEnableTamedMating (LocalVariables|GettempDino) enableMating false))
                    (:then_2
                      (Networking|ForceNetUpdate (LocalVariables|GettempDino))))
                  (else
                    (bind _asprimaldinocharacter_2 (Utilities|Casting|CastToPrimalDinoCharacterClass (Utilities|GetClass _array_element_3)))
                    (if (not (Utilities|Array|ContainsItem (LocalVariables|GetdinoClassesToIgnore) _asprimaldinocharacter_2))
                      (goto _label))))))))))))

(fn GetFilterOptions
  (Class|KismetSystemLibrary|IsRunningonServer
    (:Yes
      (if (not (Variables|Default|GetfilterCheckLocked))
        (Variables|Default|SetfilterCheckLocked true)
        (Variables|Default|SetdinoFilterOptions (Utilities|Array|MakeArray) true)
        ;[1 1 1] Disables if range is 0
        (if (> (Variables|Default|GeteffectRange) 0.0)
          ;[1 1 1] Gets all dinos in range (sorted by distance)
          (bind _returnvalue (Class|VictoryCore|ServerOctreeOverlapActorsClass (Class|Actor|GetWorld) (Transformation|GetActorLocation) (Variables|Default|GeteffectRange) "DINOPAWNS_TAMED" "/Script/ShooterGame.PrimalDinoCharacter" false))
          (bind _returnvalue_2 (Class|VictoryCore|SortActorsbyDistance (Transformation|GetActorLocation) _returnvalue))
          ;[1 1 1] Only affects owned dinos
          (bind _array_element (Utilities|Array|ForEachLoopwithBreak _returnvalue_2 :!label _label)
            (:LoopBody
              (if (== (Variables|/Script/Engine.Actor|GetTargetingTeam _array_element) (Variables|Default|GetTargetingTeam))
                (bind _asprimaldinocharacter (Utilities|Casting|CastToPrimalDinoCharacter _array_element))
                (LocalVariables|SettempDino _asprimaldinocharacter)
                ;[1 1 1] Ends search once filter options are full
                (if (< (Utilities|Array|Length (Variables|Default|GetdinoFilterOptions)) 5)
                  ;[1 1 1] Adds the dino's class to the list of options if it isn't already present
                  (bind _asprimaldinocharacter_2 (Utilities|Casting|CastToPrimalDinoCharacterClass (Utilities|GetClass (LocalVariables|GettempDino))))
                  (if (not (Utilities|Array|ContainsItem (Variables|Default|GetdinoFilterOptions) _asprimaldinocharacter_2))
                    (Utilities|Array|Add (Variables|Default|GetdinoFilterOptions) _asprimaldinocharacter_2))
                  (else
                    (goto _label Break)))))
            (:Completed
              ;[1 1 1] Updates filter options to client
              (Variables|Default|SetdinoFilterOptions (Variables|Default|GetdinoFilterOptions) true))))))))

(fn BPClientDoMultiUse
  (params (ForPC :type Player%20Controller%20Object%20Reference) (ClientUseIndex :type Integer))
  (|CallParentFunction ForPC ClientUseIndex)
  (Class|KismetSystemLibrary|SwitchNetworkMode
    (:Standalone
      _)
    (:Client
      _))
  (LocalVariables|SetplayerController ForPC)
  (switch string (Utilities|String|ToString(Integer) ClientUseIndex)
    (:90515
      ;[1 1 1] Opens filter selection menu
      (bind _asshooterplayercontroller (Utilities|Casting|CastToShooterPlayerController (LocalVariables|GetplayerController)))
      (Class|ShooterPlayerController|SetMultiUseWheelCategory _asshooterplayercontroller 91500))
    (:91501
      ;[1 1 1] Closes filter selection menu
      (bind _asshooterplayercontroller_2 (Utilities|Casting|CastToShooterPlayerController (LocalVariables|GetplayerController) :!label _label))
      (Class|ShooterPlayerController|SetMultiUseWheelCategory _asshooterplayercontroller_2 0))
    (:91502
      (goto _label))
    (:91503
      (goto _label))
    (:91504
      (goto _label))
    (:91505
      (goto _label))
    (:91506
      (goto _label))))

(fn IsDinoFilterSet
  (return (not (== "/Script/ShooterGame.PrimalDinoCharacter" (Variables|Default|GetdinoFilter)))))