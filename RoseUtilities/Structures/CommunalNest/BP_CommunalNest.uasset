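; Communal Nest structure that auto-collects same-team dropped eggs and incubates fertilized ones in its inventory.
; Server timers drive range scans, durability-based incubation and optional disabling of mating for nearby team dinos when full, using global-actor config and server hatch speed.
; Team-only multi-use entries toggle fertilized/unfertilized pickup and a species filter taken from an inventory egg.
; The filter briefly spawns that dino to read its egg classes.
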(event EventParentFirstBeginPlay
  (Utilities|FlowControl|Sequence
    (:then_0
      ;[1 1 1] Gets auto-collect range config
      (Class|KismetSystemLibrary|IsRunningonServer
        (:Yes
          (bind _globalactor (CallFunction|RUGetGlobalActor self))
          (Variables|Default|SeteffectRange (* 300 (Variables|/Game/Mods/RosesUtilities/RosesUtilities_GlobalActor.RosesUtilities_GlobalActor_C|GetCommunalNestAutoCollectRange _globalactor)) true)
          ;[1 1 1] Gets incubation rate config
          (Variables|Default|SetincubationMultiplier (Variables|/Game/Mods/RosesUtilities/RosesUtilities_GlobalActor.RosesUtilities_GlobalActor_C|GetCommunalNestIncubationRate _globalactor) true)
          ;[1 1 1] Gets disable mating when full config
          (Variables|Default|SetshouldDisableMatingWhenFull (Variables|/Game/Mods/RosesUtilities/RosesUtilities_GlobalActor.RosesUtilities_GlobalActor_C|GetCommunalNestDisableMatingWhenFull _globalactor) true)
          ;[1 1 1] Gets hatch speed from server config
          (bind _asshootergamestate (Utilities|Casting|CastToShooterGameState (Game|GetGameState)))
          (Variables|Default|SetserverEggHatchSpeedMultiplier (Variables|/Script/ShooterGame.ShooterGameState|GetEggHatchSpeedMultiplier _asshootergamestate)))))
    (:then_1
      ;[1 1 1] Restores saved visibility
      (CallFunction|OnRepEffectRange))
    (:then_2
      ;[1 1 1] Starts collect item scan, incubate eggs loops, and disable mating when full check
      (Class|KismetSystemLibrary|IsRunningonServer
        (:Yes
          (Utilities|FlowControl|Delay 0.5)
          (Utilities|Time|SetTimerbyFunctionName 0 "AutoCollectItems" 1e+01 true)
          (Utilities|FlowControl|Delay 1.0)
          (Utilities|Time|SetTimerbyFunctionName 0 "IncubateEggs" 1e+01 true)
          (if (Variables|Default|GetshouldDisableMatingWhenFull)
            (Utilities|FlowControl|Delay 1.0)
            (Utilities|Time|SetTimerbyFunctionName 0 "DisableMatingWhenFull" 6e+01 true)))))))

(fn ConstructionScript
  (|CallParentFunction))

(fn BPGetMultiUseEntries
  (params (ForPC :type Player%20Controller%20Object%20Reference) (MultiUseEntries :type Array%20of%20Multi%20Use%20Entry%20Structures))
  (bind _returnvalue (|CallParentFunction ForPC MultiUseEntries))
  (LocalVariables|SettempMultiUseEntries _returnvalue)
  (if (== (Variables|Default|GetTargetingTeam) (Variables|/Script/Engine.Actor|GetTargetingTeam ForPC))
    (Utilities|FlowControl|Sequence
      (:then_0
        ;[1 1 1] Adds a MultiUse entry to toggle auto collecting unfertilized eggs on or off
        (Utilities|Array|Add (LocalVariables|GettempMultiUseEntries) (Utilities|Struct|MakeMultiUseEntry 0 (Utilities|String|SelectString "Disable Auto-Collect Unfertilized Eggs" "Enable Auto-Collect Unfertilized Eggs" (Variables|Default|GetisAutoCollectActive_Unfertilized)) 90314 -10000)))
      (:then_1
        ;[1 1 1] Adds a MultiUse entry to toggle auto collecting fertilized eggs on or off
        (Utilities|Array|Add (LocalVariables|GettempMultiUseEntries) (Utilities|Struct|MakeMultiUseEntry 0 (Utilities|String|SelectString "Disable Auto-Collect Fertilized Eggs" "Enable Auto-Collect Fertilized Eggs" (Variables|Default|GetisAutoCollectActive_Fertilized)) 90414 -10001)))
      (:then_2
        ;[1 1 1] Adds a MultiUse entry to toggle auto collecting fertilized eggs on or off
        (bind _descriptivename (CallFunction|RUGetDescriptiveName (Variables|Default|GeteggDinoFilter)))
        (Utilities|Array|Add (LocalVariables|GettempMultiUseEntries) (Utilities|Struct|MakeMultiUseEntry 0 (Utilities|String|SelectString "Create Egg Filter" (Utilities|String|JoinStringArray (Utilities|Array|MakeArray "Remove Egg Filter (" _descriptivename ")") "") (== (Variables|Default|GeteggDinoFilter) "/Script/ShooterGame.PrimalDinoCharacter")) 90514 -10002)))
      (:then_3
        (return (LocalVariables|GettempMultiUseEntries))))
    (else
      (return (LocalVariables|GettempMultiUseEntries)))))

(fn BPTryMultiUse
  (params (ForPC :type Player%20Controller%20Object%20Reference) (UseIndex :type Integer))
  (|CallParentFunction ForPC UseIndex)
  (LocalVariables|SetplayerController ForPC)
  (Utilities|FlowControl|Sequence
    (:then_0
      (switch string (Utilities|String|ToString(Integer) UseIndex)
        (:90314
          ;[1 1 1] Toggles unfertilized auto-collect
          (Variables|Default|SetisAutoCollectActive_Unfertilized (not (Variables|Default|GetisAutoCollectActive_Unfertilized)) true))
        (:90414
          ;[1 1 1] Toggles fertilized auto-collect
          (Variables|Default|SetisAutoCollectActive_Fertilized (not (Variables|Default|GetisAutoCollectActive_Fertilized)) true))
        (:90514
          ;[1 1 1] Toggles egg filter
          (if (== (Variables|Default|GeteggDinoFilter) "/Script/ShooterGame.PrimalDinoCharacter")
            ;[1 1 1] Creates egg filter from first egg found in inventory
            (bind _returnvalue (Class|PrimalInventoryComponent|FindAllItemsOfType (Variables|Default|GetMyInventoryComponent) "/Game/PrimalEarth/CoreBlueprints/Items/Consumables/PrimalItemConsumable_Egg.PrimalItemConsumable_Egg_C" false true false false false false false))
            ;;[1 1 1] Warns player if no eggs in inventory
            (if (== (Utilities|Array|Length _returnvalue) 0)
              (CallFunction|RUMessageClient (LocalVariables|GetplayerController) "No fertilized eggs in inventory to set filter from!" "NewEnumerator1")
              (else
                ;;[1 1 1] Finds the first valid egg in inventory and sets it to filter
                (bind _array_element (Utilities|Array|ForEachLoopwithBreak _returnvalue :!label _label)
                  (:LoopBody
                    (if (!= (Variables|/Script/ShooterGame.PrimalItem|GetEggDinoClassToSpawn _array_element) 0)
                      (Variables|Default|SeteggDinoFilter (Variables|/Script/ShooterGame.PrimalItem|GetEggDinoClassToSpawn _array_element) true)
                      (goto _label Break)))
                  (:Completed
                    ;;[1 1 1] Tells player new filter or warns that no eggs in inventory were valid
                    (if (!= (Variables|Default|GeteggDinoFilter) "/Script/ShooterGame.PrimalDinoCharacter")
                      (bind _descriptivename (CallFunction|RUGetDescriptiveName (Variables|Default|GeteggDinoFilter) "/Game/PrimalEarth/Test/PrimalItemConsumable_Egg_Stego_Fertilized.PrimalItemConsumable_Egg_Stego_Fertilized"))
                      (CallFunction|RUMessageClient (LocalVariables|GetplayerController) (Utilities|String|JoinStringArray (Utilities|Array|MakeArray "Communal Nest picking up " _descriptivename " eggs") "") "NewEnumerator2")
                      ;;[1 1 1] Gets Fertilized and Unfertilized egg classes to spawn
                      (bind _returnvalue_2 (Class|PrimalDinoCharacter|SpawnDino (Class|Actor|GetWorld (LocalVariables|GetplayerController)) (Variables|Default|GeteggDinoFilter) "0,0.000000, 0" "0, 0, 0" 1.0 0 false false 0 false 1.0 0 false))
                      (Variables|Default|SeteggDinoFilterClasses (Variables|/Script/ShooterGame.PrimalDinoCharacter|GetFertilizedEggItemsToSpawn _returnvalue_2))
                      (Utilities|Array|AppendArray (Variables|Default|GeteggDinoFilterClasses) (Variables|/Script/ShooterGame.PrimalDinoCharacter|GetEggItemsToSpawn _returnvalue_2))
                      (Actor|DestroyActor _returnvalue_2)
                      (else
                        (CallFunction|RUMessageClient (LocalVariables|GetplayerController) "No valid fertilized eggs in inventory to set filter from!" "NewEnumerator1")))))))
            (else
              ;[1 1 1] Resets egg filter
              (Variables|Default|SeteggDinoFilter "/Script/ShooterGame.PrimalDinoCharacter" true)
              (CallFunction|RUMessageClient (LocalVariables|GetplayerController) "Communal Nest picking up all eggs" "NewEnumerator2"))))))
    (:then_1
      (return true))))

(fn AutoCollectItems
  (Class|KismetSystemLibrary|IsRunningonServer
    (:Yes
      ;[1 1 1] Disables if range is 0
      (if (> (Variables|Default|GeteffectRange) 0.0)
        ;[1 1 1] Gets all dropped items in range
        (if (or (Variables|Default|GetisAutoCollectActive_Fertilized) (Variables|Default|GetisAutoCollectActive_Unfertilized))
          (bind _returnvalue (Class|VictoryCore|ServerOctreeOverlapActorsClass (Class|Actor|GetWorld) (Transformation|GetActorLocation) (Variables|Default|GeteffectRange) "ALL_SPATIAL" "/Script/ShooterGame.DroppedItem" true))
          ;[1 1 1] Picks up each dropped egg in range
          (for _array_element _returnvalue
            (if (== (Variables|/Script/Engine.Actor|GetTargetingTeam _array_element) (Variables|Default|GetTargetingTeam))
              (bind _asdroppeditem (Utilities|Casting|CastToDroppedItem _array_element))
              ;[1 1 1] Filters pickup based on if Fertilized or/and Unfertilized should be picked up
              (bind _asprimalitemconsumable_egg_c (Utilities|Casting|CastToPrimalItemConsumable_Egg (Variables|/Script/ShooterGame.DroppedItem|GetMyItem _asdroppeditem)))
              (bind _isfertilized (CallFunction|RUIsEggFertilized _asprimalitemconsumable_egg_c))
              (if (Math|Boolean|ORBoolean (Math|Boolean|ANDBoolean (Variables|Default|GetisAutoCollectActive_Fertilized) (not (Variables|Default|GetisAutoCollectActive_Unfertilized)) _isfertilized) (Math|Boolean|ANDBoolean (not (Variables|Default|GetisAutoCollectActive_Fertilized)) (Variables|Default|GetisAutoCollectActive_Unfertilized) (not _isfertilized)) (and (Variables|Default|GetisAutoCollectActive_Fertilized) (Variables|Default|GetisAutoCollectActive_Unfertilized)))
                ;[1 1 1] If filter is active, only picks up matching eggs
                (bind _asprimalitem (Utilities|Casting|CastToPrimalItemClass (Utilities|GetClass _asprimalitemconsumable_egg_c)))
                (if (or (== (Variables|Default|GeteggDinoFilter) "/Script/ShooterGame.PrimalDinoCharacter") (Utilities|Array|ContainsItem (Variables|Default|GeteggDinoFilterClasses) _asprimalitem))
                  ;[1 1 1] Prevents picking up eggs that are done incubating
                  (bind _isfertilized_2 (CallFunction|RUIsEggFertilized _asprimalitemconsumable_egg_c))
                  (if _isfertilized_2
                    (if (> (Variables|/Script/ShooterGame.PrimalItem|GetItemDurability _asprimalitemconsumable_egg_c) 3.0)
                      (Utilities|FlowControl|Sequence :!label _label
                        (:then_0
                          ;[1 1 1] Stasis check
                          (if (Variables|/Script/Engine.Actor|GetbStasised _asdroppeditem)
                            (Class|Actor|Unstasis _asdroppeditem)))
                        (:then_1
                          ;[1 1 1] Adds egg to inventory and destroys dropped item actor
                          (CallFunction|RUPickupItemtoInventory _asdroppeditem (Variables|Default|GetMyInventoryComponent) (Utilities|Array|MakeArray "/Game/PrimalEarth/CoreBlueprints/Items/Consumables/PrimalItemConsumable_Egg.PrimalItemConsumable_Egg_C")))))
                    (else
                      (goto _label))))))))))))

(fn IncubateEggs
  (Networking|SwitchHasAuthority
    (:Authority
      ;[1 1 1] Gets each fertilized egg to incubate
      (for _array_element (Variables|/Script/ShooterGame.PrimalInventoryComponent|GetInventoryItems (Variables|Default|GetMyInventoryComponent))
        (bind _asprimalitemconsumable_egg_c (Utilities|Casting|CastToPrimalItemConsumable_Egg _array_element))
        (bind _isfertilized (CallFunction|RUIsEggFertilized _asprimalitemconsumable_egg_c))
        (if _isfertilized
          (LocalVariables|SeteggToIncubate _asprimalitemconsumable_egg_c)
          ;[1 1 1] Updates egg incubation
          (if (> (Variables|/Script/ShooterGame.PrimalItem|GetItemDurability (LocalVariables|GeteggToIncubate)) 1.0)
            (Variables|/Script/ShooterGame.PrimalItem|SetItemDurability (LocalVariables|GeteggToIncubate) (Math|Float|Clamp(Float) (- (Variables|/Script/ShooterGame.PrimalItem|GetItemDurability (LocalVariables|GeteggToIncubate)) (* 1e+01 (Variables|/Script/ShooterGame.PrimalItem|GetEggLoseDurabilityPerSecond (LocalVariables|GeteggToIncubate)) (Variables|/Script/ShooterGame.PrimalItem|GetExtraEggLoseDurabilityPerSecondMultiplier (LocalVariables|GeteggToIncubate)) (Variables|Default|GetincubationMultiplier) (Variables|Default|GetserverEggHatchSpeedMultiplier))) 1.0 1e+02))
            (Class|PrimalItem|UpdatedItem (LocalVariables|GeteggToIncubate) false)))))))

(fn OnRepIncubationMultiplier)

(fn DisableMatingwhenFull
  (Class|KismetSystemLibrary|IsRunningonServer
    (:Yes
      ;[1 1 1] Disables if range is 0
      (if (> (Variables|Default|GeteffectRange) 0.0)
        ;[1 1 1] Only disable mating if inventory is full
        (bind _hasemptyslots (CallFunction|RUDoesInventoryHaveEmptySlots (Variables|Default|GetMyInventoryComponent)))
        (if (not _hasemptyslots)
          ;[1 1 1] Gets all dinos in range
          (if (Variables|Default|GetshouldDisableMatingWhenFull)
            (bind _returnvalue (Class|VictoryCore|ServerOctreeOverlapActorsClass (Class|Actor|GetWorld) (Transformation|GetActorLocation) (Variables|Default|GeteffectRange) "DINOPAWNS_TAMED" (Variables|Default|GeteggDinoFilter) false))
            ;[1 1 1] Only affects owned dinos
            (for _array_element _returnvalue
              (if (== (Variables|/Script/Engine.Actor|GetTargetingTeam _array_element) (Variables|Default|GetTargetingTeam))
                (bind _asprimaldinocharacter (Utilities|Casting|CastToPrimalDinoCharacter _array_element))
                (LocalVariables|SettempDino _asprimaldinocharacter)
                ;[1 1 1] Disables mating for dino
                (Utilities|FlowControl|Sequence
                  (:then_0
                    ;;[1 1 1] Stasis check
                    (if (Variables|/Script/Engine.Actor|GetbStasised (LocalVariables|GettempDino))
                      (Class|Actor|Unstasis (LocalVariables|GettempDino))))
                  (:then_1
                    (Variables|/Script/ShooterGame.PrimalDinoCharacter|SetbEnableTamedMating (LocalVariables|GettempDino) false false))
                  (:then_2
                    (Networking|ForceNetUpdate (LocalVariables|GettempDino))))))))))))