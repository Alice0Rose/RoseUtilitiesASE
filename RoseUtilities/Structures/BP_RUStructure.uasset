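; BP_RUStructure is a base structure Blueprint for RoseUtilities, adding a toggleable effect-range mesh and persistent lock state.
; On BeginPlay, non-preview structures restore lock and range visibility, and the server polls until the RU Global Actor loads or attempts run out before firing ParentFirstBeginPlay.
; Same-team players get a Show/Hide Range multi-use entry.
; RepNotify functions update the mesh's visibility and scale.
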(event Custom|ParentFirstBeginPlay)

(event EventBeginPlay
  (if (not (Variables|Default|GetbIsPreviewStructure))
    (Utilities|FlowControl|Delay 0.2)
    (Utilities|FlowControl|Sequence
      (:then_0
        ;[1 1 1] Restores saved locked status
        (Variables|Default|SetbIsLocked (Variables|Default|GetisLockedPersistent) true)
        ;[1 1 1] Restores saved visibility
        (CallFunction|OnRepIsRangeVisible))
      (:then_1
        ;[1 1 1] Waits until Global Actor is loaded to continue BeginPlay for server, skips check for clients
        (Class|KismetSystemLibrary|IsRunningonServer
          (:Yes
            (Utilities|FlowControl|Delay 0.1 :!label _label)
            (bind _globalactor (CallFunction|RUGetGlobalActor self))
            (Utilities|IsValid _globalactor
              (:Is%20Valid
                (if (Variables|/Game/Mods/RosesUtilities/RosesUtilities_GlobalActor.RosesUtilities_GlobalActor_C|GetisLoaded _globalactor)
                  _
                  (else
                    (Variables|Default|SetglobalActorCheckCounter (+ 1 (Variables|Default|GetglobalActorCheckCounter)) :!label _label_2)
                    (if (>= (Variables|Default|GetglobalActorCheckCounter) 6000)
                      _
                      (else
                        (goto _label))))))
              (:Is%20Not%20Valid
                (goto _label_2)))
            (CallFunction|ParentFirstBeginPlay))
          (:No
            (CallFunction|ParentFirstBeginPlay)))))))

(fn ConstructionScript
  (|CallParentFunction))

(fn BPGetMultiUseEntries
  (params (ForPC :type Player%20Controller%20Object%20Reference) (MultiUseEntries :type Array%20of%20Multi%20Use%20Entry%20Structures))
  (LocalVariables|SettempMultiUseEntries MultiUseEntries)
  (if (== (Variables|Default|GetTargetingTeam) (Variables|/Script/Engine.Actor|GetTargetingTeam ForPC))
    (Utilities|FlowControl|Sequence
      (:then_0
        ;[1 1 1] Adds a MultiUse entry to show/hide range mesh
        (if (Variables|Default|GethasRangeToggle)
          (Utilities|Array|Add (LocalVariables|GettempMultiUseEntries) (Utilities|Struct|MakeMultiUseEntry 0 (Utilities|String|SelectString "Hide Range" "Show Range" (Variables|Default|GetisRangeVisible)) 985421 -100000))))
      (:then_1
        (return (LocalVariables|GettempMultiUseEntries))))
    (else
      (return (LocalVariables|GettempMultiUseEntries)))))

(fn BPTryMultiUse
  (params (ForPC :type Player%20Controller%20Object%20Reference) (UseIndex :type Integer))
  (Utilities|FlowControl|Sequence
    (:then_0
      (switch string (Utilities|String|ToString(Integer) UseIndex)
        (:601
          ;[1 1 1] Sets persistent locking on lock use
          (Variables|Default|SetisLockedPersistent (Variables|Default|GetbIsLocked) true))
        (:985421
          ;[1 1 1] Toggles effect range showing
          (Variables|Default|SetisRangeVisible (not (Variables|Default|GetisRangeVisible)) true))))
    (:then_1
      (return true))))

(fn OnRepEffectRange
  ;[1 1 1] Updates visual scale of the effect range
  (Class|KismetSystemLibrary|CanRunCosmeticEvents
    (:Yes
      (Transformation|SetRelativeScale3D (Variables|Default|GetRangeMesh) (Math|Conversions|ToVector(Float) (Variables|Default|GeteffectRange))))))

(fn OnRepIsRangeVisible
  (Rendering|SetVisibility (Variables|Default|GetRangeMesh) (Variables|Default|GetisRangeVisible) false))