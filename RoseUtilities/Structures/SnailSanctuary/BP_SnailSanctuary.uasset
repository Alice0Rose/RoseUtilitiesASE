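; Snail Sanctuary structure that passively produces snail paste into its own inventory.
; On begin play, the server reads the per-minute production rate from the RoseUtilities global actor and, after a short delay, starts a looping one-minute ProduceResources timer.
; BPUnstasis back-fills paste for the whole minutes spent in stasis, computed from the enter and exit stasis times.
; Both grants respect the inventory's item limit.
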(event `self.ParentFirstBeginPlay`
  (`|ExecutionSequence`
    (:`then_0`
      ;[1 1 1] Gets production rate config
      (`KismetSystemLibrary.IsRunningOnServer`
        (:`Yes`
          (bind _globalactor (`/Game/Mods/RosesUtilities/Functions/RosesUtilities_GlobalActorFunctions.RU_GetGlobalActor` self))
          (set `self.productionPerMinute` (`/Game/Mods/RosesUtilities/RosesUtilities_GlobalActor.SnailSanctuaryProductionPerMinute` _globalactor)))))
    (:`then_1`
      ;[1 1 1] Starts produce resources loop
      (`KismetSystemLibrary.IsRunningOnServer`
        (:`Yes`
          (`KismetSystemLibrary.Delay` 0.6)
          (`KismetSystemLibrary.K2_SetTimer` null "ProduceResources" 60.0 true))))))

(fn `BPUnstasis`
  (`PrimalInventoryComponent.BPIncrementItemTemplateQuantity` (`self.MyInventoryComponent`) "/Game/PrimalEarth/Dinos/Achatina/PrimalItemResource_SnailPaste.PrimalItemResource_SnailPaste_C" (* (`KismetMathLibrary.FFloor` (`KismetMathLibrary.Conv_DoubleToFloat` (/ (- (`self.LastExitStasisTime`) (`self.LastEnterStasisTime`)) 60.0))) (`self.productionPerMinute`)) true false true false false false null true))

(fn `ProduceResources`
  (`PrimalInventoryComponent.BPIncrementItemTemplateQuantity` (`self.MyInventoryComponent`) "/Game/PrimalEarth/Dinos/Achatina/PrimalItemResource_SnailPaste.PrimalItemResource_SnailPaste_C" (`self.productionPerMinute`) true false true false false false null true))

(fn `UserConstructionScript`
  (`parent.UserConstructionScript`))