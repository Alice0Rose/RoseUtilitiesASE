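; BP_Packager is a container structure that periodically auto-collects resources from nearby same-team structures.
; On the server it reads range and structure whitelist from the RU global actor, then a 10-second looping timer runs octree overlaps per whitelisted class.
; It transfers items matching its inventory's allowed classes, excluding woods to spare forge fuel.
; Multi-use entries toggle auto-collect and lengthen pickup once activated; activation state drives particle visibility.
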(event EventParentFirstBeginPlay
  (Utilities|FlowControl|Sequence
    (:then_0
      ;[1 1 1] Gets auto-collect range config
      (Class|KismetSystemLibrary|IsRunningonServer
        (:Yes
          (bind _globalactor (CallFunction|RUGetGlobalActor self))
          (Variables|Default|SeteffectRange (* 300 (Variables|/Game/Mods/RosesUtilities/RosesUtilities_GlobalActor.RosesUtilities_GlobalActor_C|GetPackagerAutoCollectRange _globalactor)) true)
          (Variables|Default|SetautoCollectStructureWhitelist (Variables|/Game/Mods/RosesUtilities/RosesUtilities_GlobalActor.RosesUtilities_GlobalActor_C|GetPackagerAutoCollectStructureWhitelist _globalactor) true))))
    (:then_1
      ;[1 1 1] Restores saved visibility
      (CallFunction|OnRepEffectRange)
      (CallFunction|OnRepIsActivated))
    (:then_2
      ;[1 1 1] Starts item collect scan loop
      (Class|KismetSystemLibrary|IsRunningonServer
        (:Yes
          (Utilities|FlowControl|Delay 0.1)
          (Utilities|Time|SetTimerbyFunctionName 0 "AutoCollectItems" 1e+01 true))))))

(fn ConstructionScript)

(fn BPContainerActivated
  (Variables|Default|SetisActivated true true)
  (if (not (Variables|Default|GethasBeenActivated))
    (Variables|Default|SethasBeenActivated true true)))

(fn BPTryMultiUse
  (params (ForPC :type Player%20Controller%20Object%20Reference) (UseIndex :type Integer))
  (|CallParentFunction ForPC UseIndex)
  (Utilities|FlowControl|Sequence
    (:then_0
      (switch string (Utilities|String|ToString(Integer) UseIndex)
        (:90414
          ;[1 1 1] Toggles auto-collect
          (Variables|Default|SetisAutoCollectActive (not (Variables|Default|GetisAutoCollectActive)) true))))
    (:then_1
      (return true))))

(fn BPGetMultiUseEntries
  (params (ForPC :type Player%20Controller%20Object%20Reference) (MultiUseEntries :type Array%20of%20Multi%20Use%20Entry%20Structures))
  (bind _isautocollectactive (Variables|Default|GetisAutoCollectActive))
  (bind _returnvalue (|CallParentFunction ForPC MultiUseEntries))
  (LocalVariables|SettempMultiUseEntries _returnvalue)
  (if (== (Variables|Default|GetTargetingTeam) (Variables|/Script/Engine.Actor|GetTargetingTeam ForPC))
    (Utilities|FlowControl|Sequence
      (:then_0
        (if (Variables|Default|GethasBeenActivated)
          ;[1 1 1] Extends Pickup multiuse activation timer
          (bind (_array_element _array_index) (Utilities|Array|ForEachLoopwithBreak (LocalVariables|GettempMultiUseEntries) :!label _label)
            (:LoopBody
              (if (== (.UseIndex (Utilities|Struct|BreakMultiUseEntry _array_element)) 203)
                (Utilities|Array|SetArrayElem (LocalVariables|GettempMultiUseEntries) _array_index (Utilities|Struct|MakeMultiUseEntry (.ForComponent (Utilities|Struct|BreakMultiUseEntry (Utilities|Array|Get(acopy) (LocalVariables|GettempMultiUseEntries) _array_index))) (.UseString (Utilities|Struct|BreakMultiUseEntry (Utilities|Array|Get(acopy) (LocalVariables|GettempMultiUseEntries) _array_index))) (.UseIndex (Utilities|Struct|BreakMultiUseEntry (Utilities|Array|Get(acopy) (LocalVariables|GettempMultiUseEntries) _array_index))) (.Priority (Utilities|Struct|BreakMultiUseEntry (Utilities|Array|Get(acopy) (LocalVariables|GettempMultiUseEntries) _array_index))) (.bHideFromUI (Utilities|Struct|BreakMultiUseEntry (Utilities|Array|Get(acopy) (LocalVariables|GettempMultiUseEntries) _array_index))) (.bDisableUse (Utilities|Struct|BreakMultiUseEntry (Utilities|Array|Get(acopy) (LocalVariables|GettempMultiUseEntries) _array_index))) (.bHideActivationKey (Utilities|Struct|BreakMultiUseEntry (Utilities|Array|Get(acopy) (LocalVariables|GettempMultiUseEntries) _array_index))) (.bRepeatMultiUse (Utilities|Struct|BreakMultiUseEntry (Utilities|Array|Get(acopy) (LocalVariables|GettempMultiUseEntries) _array_index))) (.bDisplayOnInventoryUI (Utilities|Struct|BreakMultiUseEntry (Utilities|Array|Get(acopy) (LocalVariables|GettempMultiUseEntries) _array_index))) (.bDisplayOnInventoryUISecondary (Utilities|Struct|BreakMultiUseEntry (Utilities|Array|Get(acopy) (LocalVariables|GettempMultiUseEntries) _array_index))) (.bHarvestable (Utilities|Struct|BreakMultiUseEntry (Utilities|Array|Get(acopy) (LocalVariables|GettempMultiUseEntries) _array_index))) (.bIsSecondaryUse (Utilities|Struct|BreakMultiUseEntry (Utilities|Array|Get(acopy) (LocalVariables|GettempMultiUseEntries) _array_index))) (.bPersistWheelOnActivation (Utilities|Struct|BreakMultiUseEntry (Utilities|Array|Get(acopy) (LocalVariables|GettempMultiUseEntries) _array_index))) (.bOverrideUseTextColor (Utilities|Struct|BreakMultiUseEntry (Utilities|Array|Get(acopy) (LocalVariables|GettempMultiUseEntries) _array_index))) (.bDisplayOnInventoryUITertiary (Utilities|Struct|BreakMultiUseEntry (Utilities|Array|Get(acopy) (LocalVariables|GettempMultiUseEntries) _array_index))) (.bClientSideOnly (Utilities|Struct|BreakMultiUseEntry (Utilities|Array|Get(acopy) (LocalVariables|GettempMultiUseEntries) _array_index))) (.bPersistWheelRequiresDirectActivation (Utilities|Struct|BreakMultiUseEntry (Utilities|Array|Get(acopy) (LocalVariables|GettempMultiUseEntries) _array_index))) (.bDrawTooltip (Utilities|Struct|BreakMultiUseEntry (Utilities|Array|Get(acopy) (LocalVariables|GettempMultiUseEntries) _array_index))) (.WheelCategory (Utilities|Struct|BreakMultiUseEntry (Utilities|Array|Get(acopy) (LocalVariables|GettempMultiUseEntries) _array_index))) (.DisableUseColor (Utilities|Struct|BreakMultiUseEntry (Utilities|Array|Get(acopy) (LocalVariables|GettempMultiUseEntries) _array_index))) (.UseTextColor (Utilities|Struct|BreakMultiUseEntry (Utilities|Array|Get(acopy) (LocalVariables|GettempMultiUseEntries) _array_index))) 3e+01 3e+01 (.ActivationSound (Utilities|Struct|BreakMultiUseEntry (Utilities|Array|Get(acopy) (LocalVariables|GettempMultiUseEntries) _array_index))) (.UseInventoryButtonStyleOverrideIndex (Utilities|Struct|BreakMultiUseEntry (Utilities|Array|Get(acopy) (LocalVariables|GettempMultiUseEntries) _array_index))) (.AdditionalButtonsIndex (Utilities|Struct|BreakMultiUseEntry (Utilities|Array|Get(acopy) (LocalVariables|GettempMultiUseEntries) _array_index)))))
                (goto _label Break))))))
      (:then_1
        ;[1 1 1] Adds a MultiUse entry to toggle auto-collect on or off
        (Utilities|Array|Add (LocalVariables|GettempMultiUseEntries) (Utilities|Struct|MakeMultiUseEntry 0 (Utilities|String|SelectString "Auto-Collect [Enabled]" "Auto-Collect [Disabled]" _isautocollectactive) 90414 -10001 false false false false false false false false false true false false false false 0 "(B=175,G=175,R=175,A=255)" (Math|Conversions|ToColor(LinearColor) (Math|Color|SelectColor "(R=0.250000,G=1.000000,B=0.250000,A=1.000000)" "(R=1.000000,G=0.250000,B=0.250000,A=1.000000)" _isautocollectactive)))))
      (:then_2
        (return (LocalVariables|GettempMultiUseEntries))))
    (else
      (return (LocalVariables|GettempMultiUseEntries)))))

(fn AutoCollectItems
  (Class|KismetSystemLibrary|IsRunningonServer
    (:Yes
      ;[1 1 1] Disables if range is 0
      (if (> (Variables|Default|GeteffectRange) 0.0)
        (if (Variables|Default|GetisAutoCollectActive)
          ;[1 1 1] Gets items allowed to be collected from the items that can be inserted into the inventory, wood is excluded from structures for forge fuel
          (LocalVariables|SetitemsToCollect (Variables|/Script/ShooterGame.PrimalInventoryComponent|GetRemoteAddItemOnlyAllowItemClasses (Variables|Default|GetMyInventoryComponent)))
          (Utilities|Array|RemoveIndex (LocalVariables|GetitemsToCollect))
          (LocalVariables|SetitemsToCollect_Structures (LocalVariables|GetitemsToCollect))
          (Utilities|Array|RemoveItem (LocalVariables|GetitemsToCollect_Structures) "/Game/PrimalEarth/CoreBlueprints/Resources/PrimalItemResource_Wood.PrimalItemResource_Wood_C")
          (Utilities|Array|RemoveItem (LocalVariables|GetitemsToCollect_Structures) "/Game/Aberration/CoreBlueprints/Resources/PrimalItemResource_FungalWood.PrimalItemResource_FungalWood_C")
          (Utilities|Array|RemoveItem (LocalVariables|GetitemsToCollect_Structures) "/Game/Extinction/CoreBlueprints/Resources/PrimalItemResource_CorruptedWood.PrimalItemResource_CorruptedWood_C")
          ;[1 1 1] Gets all the structures of each class in the config
          (for _array_element (Variables|Default|GetautoCollectStructureWhitelist)
            (bind _returnvalue (Class|VictoryCore|ServerOctreeOverlapActorsClass (Class|Actor|GetWorld) (Transformation|GetActorLocation) (Variables|Default|GeteffectRange) "STRUCTURES" _array_element false))
            (for _array_element_2 _returnvalue
              ;[1 1 1] Transfers resources to collect from all owned matching structures
              (if (== (Variables|/Script/Engine.Actor|GetTargetingTeam _array_element_2) (Variables|Default|GetTargetingTeam))
                (bind _asprimalstructureitemcontainer (Utilities|Casting|CastToPrimalStructureItemContainer _array_element_2))
                (CallFunction|RUTransferAllItems (Variables|/Script/ShooterGame.PrimalStructureItemContainer|GetMyInventoryComponent _asprimalstructureitemcontainer) (Variables|Default|GetMyInventoryComponent) (LocalVariables|GetitemsToCollect_Structures) false true false false false)))))))))

(fn OnRepIsActivated
  ;[1 1 1] Toggles SFX based on if structure is active
  (Rendering|SetVisibility (Variables|Default|GetParticles) (Variables|Default|GetisActivated) true))

(fn BPContainerDeactivated
  (Variables|Default|SetisActivated false true))